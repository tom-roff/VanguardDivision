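; DOGGIE is a dog quest target actor whose static mesh is hidden at BeginPlay and revealed by the DogQuestStart event.
; Its Lookingat event reports to the first DOGGIEQUEST actor found in the level by calling DogHelped, then hides the mesh again.
; Lookingat has no check that the quest has started, and only mesh visibility changes.
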(event `DogQuestStart`
  (`SceneComponent.SetVisibility` (`self.StaticMesh`) true false))

(event `self.ReceiveBeginPlay`
  (`SceneComponent.SetVisibility` (`self.StaticMesh`) false false))

(event `/Game/Blueprints/Interfaces/PlayerInterface.LookingAt`
  (bind _outactors (`GameplayStatics.GetAllActorsOfClass` "/Game/Blueprints/Quests/DOGGIEQUEST.DOGGIEQUEST_C"))
  (`/Game/Blueprints/Quests/DOGGIEQUEST.DogHelped` (`|GetArrayItem` _outactors))
  (`SceneComponent.SetVisibility` (`self.StaticMesh`) false false))

(fn `UserConstructionScript`)