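; VariousFuncs holds a utility function, FindLowestValue, that finds the nearest actor of a given class to an origin actor.
; It gathers all actors of that class and linearly scans their distances, keeping any below the stored ClosestDistance, which the graph does not initialize.
; It prints the winner's display name, then returns that actor and its distance.
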(fn `FindLowestValue`
  (params (ActorClass :type "Actor Class Reference") (`Current Actor (Self, Origin)` :type "Actor Object Reference"))
  (returns (`Closest Actor` :type "Actor Object Reference") (`Distance to Closest Actor` :type "Float (double-precision)"))
  (locals (`Closest Distance` :type "Float (double-precision)" :default 20000000.0) (ClosestActor :type "Actor Object Reference"))
  (bind _outactors (`GameplayStatics.GetAllActorsOfClass` null ActorClass))
  (for _array_element _outactors
    (bind _returnvalue (`Actor.GetDistanceTo` `Current Actor (Self, Origin)` _array_element))
    (if (< _returnvalue (`local.Closest Distance`))
      (set `local.ClosestActor` _array_element)
      (set `local.Closest Distance` _returnvalue)))
  (`KismetSystemLibrary.PrintString` null (`KismetSystemLibrary.GetDisplayName` (`local.ClosestActor`)))
  (return (`local.ClosestActor`) (`local.Closest Distance`)))