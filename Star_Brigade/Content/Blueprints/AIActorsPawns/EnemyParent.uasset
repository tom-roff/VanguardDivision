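; Base enemy character for the wave game, with health scaled by game mode difficulty in the construction script.
; Looping timers flag low-speed blockage on the Blackboard and tick plasma coil damage while in range.
; KillBot removes the controller, ragdolls with impulse and explosion, triggers killer perks, pays currency to all players and credits the killer.
; Custom-depth stencil drives highlights, including perk-based threat outlines; destruction deregisters it from active enemies.
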(event `self.ReceiveBeginPlay`
  (`self.CreateOutline`))

(event `SetParticleVisMulti`
  (params (`Hidden?` :type Boolean))
  ;[1 1 1] Plasma Effects
  (if (not (`self.IsDead?`))
    (`SceneComponent.SetHiddenInGame` (`self.PlasmaFX`) `Hidden?` false)))

(event `StartCheckingForObjInWay`
  ;[1 1 1] Check for Placeables
  (bind _returnvalue (`KismetSystemLibrary.K2_SetTimerDelegate` (delegate `CheckSpeed`) 0.5 true))
  (set `self.CheckForObjTimer` _returnvalue))

(event `DealPlasmaDamage`
  (params (`# of times to hit` :type Integer) (`Coil Damage` :type "Float (double-precision)") (`Time Between Damage Ticks` :type "Float (double-precision)") (EventInstigator :type "Controller Object Reference") (DamageCauser :type "Actor Object Reference"))
  ;[1 1 1] Plasma Coil Handling
  (`self.SetParticleVisMulti` false)
  (set `self.#ofTimestoHitWithPlasma` `# of times to hit`)
  (if (not (`KismetSystemLibrary.K2_IsValidTimerHandle` (stale `DealPlasmaDamage` _returnvalue)))
    (bind _returnvalue (`KismetSystemLibrary.K2_SetTimerDelegate` (delegate `ApplyPlasmaDamage`) `Time Between Damage Ticks` true))))

(event `CheckSpeed`
  (bind _returnvalue (`AIBlueprintHelperLibrary.GetBlackboard` self))
  ;[1 1 1] Check for Placeables
  (`KismetSystemLibrary.PrintString` "Checking for blocked object")
  (if (and (< (`KismetMathLibrary.VSize` (`MovementComponent.Velocity` (`self.CharacterMovement`))) 200.0) (not (`self.IsSlowedByForceZone?`)))
    (`/Engine/EditorBlueprintResources/StandardMacros.IsValid` _returnvalue
      (:`Is Valid`
        (`BlackboardComponent.SetValueAsBool` _returnvalue "IsBlockedByObj?" true)
        (`MovementComponent.StopMovementImmediately` (`self.CharacterMovement`))))
    (else
      (`BlackboardComponent.SetValueAsBool` _returnvalue "IsBlockedByObj?" false))))

(event `ApplyPlasmaDamage`
  ;[1 1 1] Plasma Coil Handling
  (if (`self.IsInPlasmaRange?`)
    (`GameplayStatics.ApplyDamage` self (stale `DealPlasmaDamage` `Coil Damage`) (stale `DealPlasmaDamage` EventInstigator) (stale `DealPlasmaDamage` DamageCauser))
    (else
      (`KismetSystemLibrary.K2_ClearAndInvalidateTimerHandle` (stale `DealPlasmaDamage` _returnvalue))
      (`self.SetParticleVisMulti` true))))

(event `StopCheckingForObjInWay`
  (bind _returnvalue (`AIBlueprintHelperLibrary.GetBlackboard` self))
  ;[1 1 1] Check for Placeables
  (`KismetSystemLibrary.K2_ClearAndInvalidateTimerHandle` (`self.CheckForObjTimer`))
  (`/Engine/EditorBlueprintResources/StandardMacros.IsValid` _returnvalue
    (:`Is Valid`
      (`BlackboardComponent.SetValueAsBool` _returnvalue "IsBlockedByObj?" false))))

(event `self.ReceiveDestroyed`
  ;[1 1 1] When destroyed, tell the game mode that we're no longer an active enemy
  (bind _aswave_gmupdated (cast `/Game/Blueprints/Gameplay/WaveGMUpdated` (`GameplayStatics.GetGameMode`)))
  (`KismetArrayLibrary.Array_RemoveItem` (`/Game/Blueprints/Gameplay/WaveGMUpdated.ActiveEnemies` _aswave_gmupdated) self))

(event `KillBot`
  (params (`Instigated Controller` :type "PlayerController Object Reference") (`Currency Reward` :type Integer) (`Wave Cash Reward` :type Integer) (`Damage Causer` :type "Actor Object Reference"))
  (bind _asplayer_state_1main (cast `/Game/Blueprints/AllLevels/PlayerState1Main` (`Controller.PlayerState` `Instigated Controller`) :!pure true))
  ;[1 1 1] Handle Bot death
  (`self.EndHighlight`)
  (`self.SetParticleVisMulti` true)
  (bind _asaicontroller (cast `AIController` (`self.GetController`)))
  (`Controller.UnPossess` _asaicontroller)
  (`self.K2_DestroyActor` _asaicontroller)
  (`MovementComponent.StopMovementImmediately` (`self.CharacterMovement`))
  (`self.DoDeathMulti` (`self.Hit Bone`) (`self.K2_GetActorLocation` (select `bool` (`KismetSystemLibrary.IsValid` `Damage Causer`) :`false` (`GameplayStatics.GetPlayerCharacter` 0) :`true` `Damage Causer` :!type "Actor Object Reference")))
  (if (`self.IsSpecial?`)
    (`self.SpecialDeathCheck` `Instigated Controller`))
  (`self.NormalPerkCheck` `Instigated Controller`)
  (`PrimitiveComponent.SetCollisionResponseToChannel` (`self.Mesh`) "ECC_GameTraceChannel2" "ECR_Ignore")
  (bind _outactors (`GameplayStatics.GetAllActorsOfClass` "/Game/TrueFPP/TrueFirstPersonCharacter.TrueFirstPersonCharacter_C"))
  (for _array_element _outactors
    (bind (_equippedwep1new _class _equippedweapon2 _equippedtool _currency) (break `/Game/Blueprints/AllLevels/Variables/Structs/PlayerInfoBase` (`/Game/TrueFPP/TrueFirstPersonCharacter.PlayerInfo` _array_element)))
    (set `/Game/TrueFPP/TrueFirstPersonCharacter.PlayerInfo` (make `/Game/Blueprints/AllLevels/Variables/Structs/PlayerInfoBase` _equippedwep1new _class _equippedweapon2 _equippedtool (+ _currency `Currency Reward`)) _array_element)
    (`/Game/TrueFPP/TrueFirstPersonCharacter.MoneyUpdate` _array_element `Currency Reward`))
  (set `self.IsDead?` true)
  (`/Engine/EditorBlueprintResources/StandardMacros.IsValid` `Instigated Controller`
    (:`Is Valid`
      (set `/Game/Blueprints/AllLevels/PlayerState1Main.CurrentWaveCash` (+ (`/Game/Blueprints/AllLevels/PlayerState1Main.CurrentWaveCash` _asplayer_state_1main) `Wave Cash Reward`) _asplayer_state_1main)
      (set `/Game/Blueprints/AllLevels/PlayerState1Main.Kills` (+ (`/Game/Blueprints/AllLevels/PlayerState1Main.Kills` _asplayer_state_1main) 1) _asplayer_state_1main))
    (:`Is Not Valid`
      _))
  (`KismetSystemLibrary.Delay` 5.0)
  (`self.K2_DestroyActor`))

(event `DoDeathMulti`
  (params (BoneName :type Name) (Start :type "Vector Structure (by ref)"))
  (bind _mesh (`self.Mesh`))
  (bind _mesh_2 (`self.Mesh`))
  ;[1 1 1] Handle Bot death
  (`SkeletalMeshComponent.Stop` (`self.Mesh`))
  (`PrimitiveComponent.SetSimulatePhysics` _mesh_2 true)
  (`SkeletalMeshComponent.SetPhysicsBlendWeight` _mesh_2 1.0)
  (`PrimitiveComponent.SetCollisionEnabled` (`self.CapsuleComponent`) "NoCollision")
  (`PrimitiveComponent.SetCollisionEnabled` _mesh "QueryAndPhysics")
  (`self.DoExplosion`)
  (`CharacterMovementComponent.SetAvoidanceEnabled` (`self.CharacterMovement`) false)
  (`KismetSystemLibrary.Delay` 0.05)
  (`PrimitiveComponent.AddImpulseAtLocation` (`self.Mesh`) (+ (* (`KismetMathLibrary.GetForwardVector` (`KismetMathLibrary.FindLookAtRotation` Start (`self.K2_GetActorLocation`))) 3000000.0) (0.0 0.0 1000000.0)) (`SceneComponent.GetSocketLocation` _mesh BoneName) BoneName))

(event `DoExplosion`
  ;[1 1 1] Death Explosion
  (`GameplayStatics.SpawnEmitterAttached` "/Game/Particles/VFX_Toolkit_V1/ParticleSystems/356Days/Par_MatraBoom_01.Par_MatraBoom_01" (`self.Mesh`) "None" (0.0 0.0 60.0) (struct) (0.4 0.4 0.9))
  (`GameplayStatics.PlaySoundAtLocation` "/Game/Audio/SoundFX/zapsplat_explosion_med_large_71697.zapsplat_explosion_med_large_71697" (`SceneComponent.K2_GetComponentLocation` (`self.Mesh`)) (struct) 0.3 0.9 0.0 "/Game/Audio/Attenuations/BaseAtten.BaseAtten" null self))

(event `StartHighlight`
  (params (HighlightColor :type Integer))
  (bind _mesh (`self.Mesh`))
  ;[1 1 1] Highlight
  (`PrimitiveComponent.SetRenderCustomDepth` _mesh true)
  (`PrimitiveComponent.SetCustomDepthStencilValue` _mesh HighlightColor))

(event `SpecialDeathCheck`
  (params (`Instigated Controller` :type "Controller Object Reference"))
  ;[1 1 1] Special Perks Triggering
  (bind _astrue_first_person_character (cast `/Game/TrueFPP/TrueFirstPersonCharacter` (`Controller.K2_GetPawn` `Instigated Controller`)))
  (bind _purchasedperks (`/Game/TrueFPP/TrueFirstPersonCharacter.PurchasedPerks` _astrue_first_person_character))
  (if (`KismetArrayLibrary.Array_Contains` _purchasedperks "NewEnumerator5")
    (`/Game/TrueFPP/TrueFirstPersonCharacter.HealPlayer` _astrue_first_person_character (`self.AmountToHealWithMorphineCell`))
    (elif (`KismetArrayLibrary.Array_Contains` _purchasedperks "NewEnumerator9")
      (bind _asgun_parent (cast `/Game/Blueprints/Weapons/GunParent` (`/Game/TrueFPP/TrueFirstPersonCharacter.CurrentWeaponInHand` _astrue_first_person_character)))
      (`/Game/Blueprints/Weapons/GunParent.OverloaderFireRate` _asgun_parent))))

(event `EndHighlight`
  ;[1 1 1] Highlight
  (`PrimitiveComponent.SetRenderCustomDepth` (`self.Mesh`) false))

(event `CreateOutline`
  ;[1 1 1] Highlight
  (`/Engine/EditorBlueprintResources/ActorMacros.Switch Has Authority`
    (:`Authority`
      (bind _outactors (`GameplayStatics.GetAllActorsOfClass` "/Game/TrueFPP/TrueFirstPersonCharacter.TrueFirstPersonCharacter_C"))
      (for _array_element _outactors
        (if (`KismetArrayLibrary.Array_Contains` (`/Game/TrueFPP/TrueFirstPersonCharacter.PurchasedPerks` _array_element) "NewEnumerator2")
          (bind _asplayer_controller_main (cast `/Game/Blueprints/AllLevels/PlayerControllerMain` (`self.GetController` _array_element)))
          (`/Game/Blueprints/AllLevels/PlayerControllerMain.SetThreatHudOutline` _asplayer_controller_main true (`self.Mesh`)))))))

(event `PlayHitSound`
  (params (`CritShot?` :type Boolean))
  ;[1 1 1] Hit Sound
  (`KismetSystemLibrary.Delay` 0.1)
  (`GameplayStatics.PlaySoundAtLocation` (select `bool` `CritShot?` :`false` "/Game/Audio/SoundFX/MetalSounds/Hit6.Hit6" :`true` "/Game/Audio/SoundFX/MetalSounds/Hit4.Hit4" :!type "SoundBase Object Reference") (`self.K2_GetActorLocation`) (struct) 1.0 1.0 0.0 "/Game/Audio/Attenuations/BaseAtten.BaseAtten" null self))

(event `NormalPerkCheck`
  (params (`Instigated Controller` :type "Controller Object Reference"))
  ;[1 1 1] Normal Death (Currently Just Siphoner)
  (bind _astrue_first_person_character (cast `/Game/TrueFPP/TrueFirstPersonCharacter` (`Controller.K2_GetPawn` `Instigated Controller`)))
  (if (`KismetArrayLibrary.Array_Contains` (`/Game/TrueFPP/TrueFirstPersonCharacter.PurchasedPerks` _astrue_first_person_character) "NewEnumerator12")
    (`/Game/TrueFPP/TrueFirstPersonCharacter.HealPlayer` _astrue_first_person_character 2)))

(fn `UserConstructionScript`
  (bind _aswave_gmupdated (cast `/Game/Blueprints/Gameplay/WaveGMUpdated` (`GameplayStatics.GetGameMode`)))
  (switch `/Game/Blueprints/AllLevels/Variables/Enums/Difficulties` (`/Game/Blueprints/Gameplay/WaveGMUpdated.Difficulty` _aswave_gmupdated)
    (:`NewEnumerator0`
      (set `self.Health` (* (`self.Health`) 0.666667)))
    (:`NewEnumerator1`
      (set `self.Health` (`self.Health`)))
    (:`NewEnumerator2`
      (set `self.Health` (* (`self.Health`) 1.333333)))
    (:`NewEnumerator3`
      (set `self.Health` (* (`self.Health`) 1.5)))))