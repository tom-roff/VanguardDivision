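; Behavior tree task that finds the closest living, non-downed player character to the AI-controlled pawn.
; It loops over all TrueFirstPersonCharacter actors, skips dead or downed ones, and keeps the nearest within a very large starting distance.
; The result is written to the ClosestObj blackboard key, and the task always finishes successfully, even when no player qualifies.
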(event `self.ReceiveExecuteAI`
  (params (OwnerController :type "AIController Object Reference") (ControlledPawn :type "Pawn Object Reference"))
  (bind _outactors (`GameplayStatics.GetAllActorsOfClass` "/Game/TrueFPP/TrueFirstPersonCharacter.TrueFirstPersonCharacter_C"))
  (set `self.Closest Distance` 1000000.0)
  (for _array_element _outactors
    (if (not (or (`/Game/TrueFPP/TrueFirstPersonCharacter.IsDEAD?` _array_element) (`/Game/TrueFPP/TrueFirstPersonCharacter.IsDowned?` _array_element)))
      (bind _returnvalue (`Actor.GetDistanceTo` ControlledPawn _array_element))
      (if (< _returnvalue (`self.Closest Distance`))
        (set `self.ClosestPlayer` _array_element)
        (set `self.Closest Distance` _returnvalue))))
  (`BTFunctionLibrary.SetBlackboardValueAsObject` (`self.ClosestObj`) (`self.ClosestPlayer`))
  (`self.FinishExecute` true))