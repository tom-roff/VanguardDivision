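; WidgetFuncs is a set of shared UI helpers for interact prompts, notifications and input-mode switching.
; ShowInteractWB forwards prompt text to the given controller.
; ShowGenericMessageUI removes any valid notification it references and creates a new one, treating magenta as a sentinel that keeps the default text color.
; EnterUIMode and ExitUIMode toggle cursor, input mode and player-zero character input, with entry also stopping movement.
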(fn `EnterUIMode`
  (params (InWidgetToFocus :type "Widget Object Reference"))
  (bind _returnvalue (`GameplayStatics.GetPlayerController` null))
  (bind _returnvalue_2 (`GameplayStatics.GetPlayerCharacter` null))
  (`WidgetBlueprintLibrary.SetInputMode_UIOnlyEx` _returnvalue InWidgetToFocus)
  (set `PlayerController.bShowMouseCursor` true _returnvalue)
  (`Actor.DisableInput` _returnvalue_2 _returnvalue)
  (`MovementComponent.StopMovementImmediately` (`Character.CharacterMovement` _returnvalue_2)))

(fn `ExitUIMode`
  (bind _returnvalue (`GameplayStatics.GetPlayerController` null))
  (`WidgetBlueprintLibrary.SetInputMode_GameOnly` _returnvalue)
  (set `PlayerController.bShowMouseCursor` false _returnvalue)
  (`Actor.EnableInput` (`GameplayStatics.GetPlayerCharacter` null) _returnvalue))

(fn `ShowGenericMessageUI`
  (params (`Text To Show` :type Text) (`Text Color` :type "SlateColor Structure"))
  (returns (`WB Created` :type "/Game/UI_elements/Notifications/BaseNotificationUI Object Reference"))
  (`/Engine/EditorBlueprintResources/StandardMacros.IsValid` (stale _returnvalue)
    (:`Is Valid`
      (`Widget.RemoveFromParent` (stale _returnvalue)))
    (:`Is Not Valid`
      _))
  (bind _returnvalue (`|CreateWidget` "/Game/UI_elements/Notifications/BaseNotificationUI.BaseNotificationUI_C" (`GameplayStatics.GetPlayerController` null)))
  (`UserWidget.AddToViewport` _returnvalue 0)
  (set `/Game/UI_elements/Notifications/BaseNotificationUI.Text To Show` `Text To Show` _returnvalue)
  (if (!= (`.SpecifiedColor` (break `SlateColor` `Text Color`)) (struct :`R` 1.0 :`B` 1.0 :`A` 1.0))
    (set `/Game/UI_elements/Notifications/BaseNotificationUI.Text Color` `Text Color` _returnvalue))
  (return _returnvalue))

(fn `ShowInteractWB`
  (params (TextToShow :type Text) (Controller :type "/Game/Blueprints/AllLevels/PlayerControllerMain Object Reference"))
  (returns (`WB Created` :type "/Game/UI_elements/GameplayWBs/BaseLookingAtUI Object Reference"))
  (`/Engine/EditorBlueprintResources/StandardMacros.IsValid` Controller
    (:`Is Valid`
      (bind _wb_created (`/Game/Blueprints/AllLevels/PlayerControllerMain.ShowInteractWB` Controller TextToShow))
      (return _wb_created))))