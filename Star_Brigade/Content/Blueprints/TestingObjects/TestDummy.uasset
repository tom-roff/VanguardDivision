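; Test dummy actor that takes damage, displays its health and can be reset, playing a looping idle animation.
; AnyDamage reduces Health and, at zero, a DoOnce drops the actor 60 units and flags it dead.
; The Lookingat event restores health, and for a dead dummy also raises it back up and re-arms the DoOnce.
; Tick writes current Health to a TextRender every frame.
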(event `self.ReceiveBeginPlay`
  (`SkeletalMeshComponent.PlayAnimation` (`self.SkeletalMesh`) "/Game/Mannequin/Animations/ThirdPersonIdle.ThirdPersonIdle" true))

(event `self.ReceiveAnyDamage`
  (params (Damage :type "Float (single-precision)") (DamageType :type "DamageType Object Reference") (InstigatedBy :type "Controller Object Reference") (DamageCauser :type "Actor Object Reference"))
  (bind _output_get (set `self.Health` (- (`self.Health`) Damage)))
  (if (<= _output_get 0.0)
    (`/Engine/EditorBlueprintResources/StandardMacros.DoOnce` false :!label _label
      (:`Completed`
        (`self.K2_SetActorLocation` (- (`self.K2_GetActorLocation`) (0.0 0.0 60.0)))
        (set `self.IsDead?` true)))))

(event `self.ReceiveTick`
  (params (DeltaSeconds :type "Float (single-precision)"))
  (`TextRenderComponent.K2_SetText` (`self.TextRender`) (`KismetTextLibrary.Conv_DoubleToText` (`self.Health`) "HalfToEven")))

(event `/Game/Blueprints/Interfaces/PlayerInterface.LookingAt`
  (params (LookingAtController :type "PlayerController Object Reference"))
  (if (`self.IsDead?`)
    (set `self.IsDead?` false)
    (set `self.Health` 60.0)
    (`self.K2_SetActorLocation` (- (`self.K2_GetActorLocation`) (0.0 0.0 -60.0)))
    (goto _label :!via `Reset`)
    (else
      (set `self.Health` 60.0))))

(fn `UserConstructionScript`)