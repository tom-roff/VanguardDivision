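; Multiplayer game mode that tracks connected players and keeps the game state and each player's party UI in sync as people join or leave.
; Login registers with the game state, then after a short delay refreshes health bars and announces the newcomer to others.
; Logout destroys the player state, refreshes party info and announces the leaver by Steam name.
; A travel event tells clients to change map, switching characters to UI-only input and disabling movement.
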(event `self.K2_PostLogin`
  (params (NewPlayer :type "PlayerController Object Reference"))
  ;[1 1 1] Logging in Stuffs
  (`KismetArrayLibrary.Array_Add` (`self.ConnectedPlayersGM`) NewPlayer)
  (bind _asgame_state_vdupdated (cast `/Game/Blueprints/AllLevels/GameStateVDUpdated` (`GameplayStatics.GetGameState`)))
  (`/Game/Blueprints/AllLevels/GameStateVDUpdated.RegisterLoginGameState` _asgame_state_vdupdated (`Controller.PlayerState` NewPlayer))
  (`self.RegisterLoginGamemode` NewPlayer))

(event `RegisterLoginGamemode`
  (params (`Joining Controller` :type "PlayerController Object Reference"))
  ;[1 1 1] Logging in Stuffs
  (`KismetSystemLibrary.Delay` 2.0)
  (for _array_element (`self.ConnectedPlayersGM`)
    (bind _asplayer_controller_main (cast `/Game/Blueprints/AllLevels/PlayerControllerMain` _array_element))
    (`/Game/Blueprints/AllLevels/PlayerControllerMain.SetPlayerHealthBarsArray` _asplayer_controller_main)
    (`/Game/Blueprints/AllLevels/PlayerControllerMain.SetHealthBarNamesAndSetPartyInfoVis` _asplayer_controller_main)
    (if (!= _array_element `Joining Controller`)
      (`/Game/Blueprints/AllLevels/PlayerControllerMain.AddJoinedLeaveMessage` _asplayer_controller_main true (`PlayerState.GetPlayerName` (`Controller.PlayerState` `Joining Controller`))))))

(event `self.K2_OnLogout`
  (params (ExitingController :type "Controller Object Reference"))
  (bind _asplayer_controller (cast `PlayerController` ExitingController :!pure true))
  ;[1 1 1] Logging in Stuffs
  (bind _asgame_state_vdupdated (cast `/Game/Blueprints/AllLevels/GameStateVDUpdated` (`GameplayStatics.GetGameState`)))
  (`/Game/Blueprints/AllLevels/GameStateVDUpdated.RegisterLogout` _asgame_state_vdupdated null)
  (`self.K2_DestroyActor` (`Controller.PlayerState` ExitingController))
  (`KismetArrayLibrary.Array_RemoveItem` (`self.ConnectedPlayersGM`) _asplayer_controller)
  (bind _outactors (`GameplayStatics.GetAllActorsOfClass` "/Game/Blueprints/AllLevels/PlayerControllerMain.PlayerControllerMain_C"))
  (for _array_element _outactors
    (`/Game/Blueprints/AllLevels/PlayerControllerMain.SetHealthBarNamesAndSetPartyInfoVis` _array_element)
    (if (!= _array_element ExitingController)
      (bind _returnvalue (`AdvancedSteamFriendsLibrary.GetSteamPersonaName` (`AdvancedSessionsLibrary.GetUniqueNetID` _asplayer_controller)))
      (`/Game/Blueprints/AllLevels/PlayerControllerMain.AddJoinedLeaveMessage` _array_element false _returnvalue))))

(event `TellClientsToTravelMap`
  (for _array_element (`self.ConnectedPlayersGM`)
    (bind _asplayer_controller_main (cast `/Game/Blueprints/AllLevels/PlayerControllerMain` _array_element))
    (`/Game/Blueprints/AllLevels/PlayerControllerMain.ClientsTravel` _asplayer_controller_main))
  (bind _outactors (`GameplayStatics.GetAllActorsOfClass` "/Game/TrueFPP/TrueFirstPersonCharacter.TrueFirstPersonCharacter_C"))
  (for _array_element_2 _outactors
    (`WidgetBlueprintLibrary.SetInputMode_UIOnlyEx` (cast `PlayerController` (`Pawn.GetController` _array_element_2) :!pure true) null)
    (`CharacterMovementComponent.DisableMovement` (`Character.CharacterMovement` _array_element_2))))

(fn `UserConstructionScript`)