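; Function library of dissolve and condense effects that swap an actor's mesh materials for an erode material.
; Step 1 functions fill one dynamic ErodeMat1_Inst with textures and color, apply it to every non-widget mesh slot, and return it.
; Dissolve also disables collision; condense sets ErodeValue to zero.
; CondenseStep2 and CondenseSetMat assign caller-supplied materials by mesh index, with step 2, named for a post-delay call, also handling extra slots.
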(fn `CondenseSetMat`
  (params (Actor :type "Actor Object Reference") (Material :type "MaterialInterface Object Reference") (Material1 :type "MaterialInterface Object Reference") (Material2 :type "MaterialInterface Object Reference") (Material3 :type "MaterialInterface Object Reference"))
  (locals (DynMatInst :type "MaterialInstanceDynamic Object Reference"))
  (for (_array_element _array_index) (`Actor.K2_GetComponentsByClass` Actor "/Script/Engine.MeshComponent")
    (if (!= (`GameplayStatics.GetObjectClass` _array_element) "/Script/UMG.WidgetComponent")
      (switch `int` _array_index
        (:`Default`
          (`PrimitiveComponent.SetMaterial` _array_element 0 Material :!label _label))
        (:`0`
          (goto _label))
        (:`1`
          (`PrimitiveComponent.SetMaterial` _array_element 0 Material1))
        (:`2`
          (`PrimitiveComponent.SetMaterial` _array_element 0 Material2))
        (:`3`
          (`PrimitiveComponent.SetMaterial` _array_element 0 Material3))))))

(fn `CondenseStep1`
  (params (PreviousBaseColor :type "Texture Object Reference") (PreviousRoughness :type "Texture Object Reference") (PreviousNormal :type "Texture Object Reference") (Color :type "LinearColor Structure") (Actor :type "Actor Object Reference") (`Material of Mesh 1` :type "MaterialInterface Object Reference") (`Material of Mesh 2` :type "MaterialInterface Object Reference") (`Material of Mesh 3` :type "MaterialInterface Object Reference") (`Material of Mesh 4` :type "MaterialInterface Object Reference"))
  (returns (Actor_ :type "Actor Object Reference") (`Material of Mesh 1_` :type "MaterialInterface Object Reference") (`Material of Mesh 2_` :type "MaterialInterface Object Reference") (`Material of Mesh 3_` :type "MaterialInterface Object Reference") (`Material of Mesh 4_` :type "MaterialInterface Object Reference") (`Dyn Mat Inst1` :type "MaterialInstanceDynamic Object Reference"))
  (locals (`Dyn Mat Inst` :type "MaterialInstanceDynamic Object Reference"))
  ;[1 1 1] Condense an Object
  (bind _returnvalue (`KismetMaterialLibrary.CreateDynamicMaterialInstance` null "/Game/Materials/TransitionMat/ErodeMat1_Inst.ErodeMat1_Inst"))
  (bind _output_get (set `local.Dyn Mat Inst` _returnvalue))
  (`self.SetParams` PreviousBaseColor PreviousRoughness PreviousNormal _output_get Color)
  (for _array_element (`Actor.K2_GetComponentsByClass` Actor "/Script/Engine.MeshComponent")
    (if (!= (`GameplayStatics.GetObjectClass` _array_element) "/Script/UMG.WidgetComponent")
      (for _index (range (+ (`PrimitiveComponent.GetNumMaterials` _array_element) 1))
        (`PrimitiveComponent.SetMaterial` _array_element _index (`local.Dyn Mat Inst`)))))
  (`MaterialInstanceDynamic.SetScalarParameterValue` (`local.Dyn Mat Inst`) "ErodeValue" 0.0)
  (return Actor `Material of Mesh 1` `Material of Mesh 2` `Material of Mesh 3` `Material of Mesh 4` _returnvalue))

(fn `CondenseStep2(After105SDelay)`
  (params (Actor :type "Actor Object Reference") (`Material 1` :type "MaterialInterface Object Reference") (`Mesh 2 Material` :type "MaterialInterface Object Reference") (`Mesh 3 Material` :type "MaterialInterface Object Reference") (`Mesh 4 Material` :type "MaterialInterface Object Reference") (`Mesh 1 Alt Mat 1` :type "MaterialInterface Object Reference") (`Mesh 2 2 Alt Mat 1` :type "MaterialInterface Object Reference") (`Mesh 2 Alt Mat 2` :type "MaterialInterface Object Reference") (`Mesh 1 Alt Mat 2` :type "MaterialInterface Object Reference"))
  (for (_array_element _array_index) (`Actor.K2_GetComponentsByClass` Actor "/Script/Engine.MeshComponent")
    (if (!= (`GameplayStatics.GetObjectClass` _array_element) "/Script/UMG.WidgetComponent")
      (switch `int` _array_index
        (:`Default`
          (bind _returnvalue (`PrimitiveComponent.GetNumMaterials` _array_element))
          (for _index (range (+ _returnvalue 1)) :!label _label
            (switch `int` _index
              (:`0`
                (`PrimitiveComponent.SetMaterial` _array_element _index `Material 1`))
              (:`1`
                (`PrimitiveComponent.SetMaterial` _array_element _index `Mesh 1 Alt Mat 1`))
              (:`2`
                (`PrimitiveComponent.SetMaterial` _array_element _index `Mesh 1 Alt Mat 2`)))))
        (:`0`
          (goto _label))
        (:`1`
          (for _index_2 (range (+ _returnvalue 1))
            (if (== _index_2 1)
              (`PrimitiveComponent.SetMaterial` _array_element _index_2 `Mesh 2 2 Alt Mat 1`)
              (elif (== _index_2 2)
                (`PrimitiveComponent.SetMaterial` _array_element _index_2 `Mesh 2 Alt Mat 2`)
                (else
                  (`PrimitiveComponent.SetMaterial` _array_element _index_2 `Mesh 2 Material`))))))
        (:`2`
          (for _index_3 (range (+ _returnvalue 1))
            (`PrimitiveComponent.SetMaterial` _array_element _index_3 `Mesh 3 Material`)))
        (:`3`
          (for _index_4 (range (+ _returnvalue 1))
            (`PrimitiveComponent.SetMaterial` _array_element _index_4 `Mesh 4 Material`)))))))

(fn `DissolveStep1`
  (params (Actor :type "Actor Object Reference") (BaseColor :type "Texture Object Reference") (Roughness :type "Texture Object Reference") (Normal :type "Texture Object Reference") (Color :type "LinearColor Structure") (Material :type "MaterialInterface Object Reference") (`Material of Mesh 2` :type "MaterialInterface Object Reference") (`Material of Mesh 3` :type "MaterialInterface Object Reference") (`Material of Mesh 4` :type "MaterialInterface Object Reference"))
  (returns (Actor_ :type "Actor Object Reference") (`Material of Mesh 1_` :type "MaterialInterface Object Reference") (`Material of Mesh 2_` :type "MaterialInterface Object Reference") (`Material of Mesh 3_` :type "MaterialInterface Object Reference") (`Material of Mesh 4_` :type "MaterialInterface Object Reference") (`Dyn Mat Inst1` :type "MaterialInstanceDynamic Object Reference"))
  (`/Engine/EditorBlueprintResources/StandardMacros.IsValid` Actor
    (:`Is Valid`
      (`Actor.SetActorEnableCollision` Actor false)
      (bind _returnvalue (`KismetMaterialLibrary.CreateDynamicMaterialInstance` null "/Game/Materials/TransitionMat/ErodeMat1_Inst.ErodeMat1_Inst"))
      (`self.SetParams` BaseColor Roughness Normal _returnvalue Color)
      (for _array_element (`Actor.K2_GetComponentsByClass` Actor "/Script/Engine.MeshComponent")
        (if (!= (`GameplayStatics.GetObjectClass` _array_element) "/Script/UMG.WidgetComponent")
          (for _index (range (+ (`PrimitiveComponent.GetNumMaterials` _array_element) 1))
            (`PrimitiveComponent.SetMaterial` _array_element _index _returnvalue))))
      (return Actor Material `Material of Mesh 2` `Material of Mesh 3` `Material of Mesh 4` _returnvalue))))

(fn `SetParams`
  (params (BaseColor :type "Texture Object Reference") (Roughness :type "Texture Object Reference") (Normal :type "Texture Object Reference") (`Dyn Mat Inst` :type "MaterialInstanceDynamic Object Reference") (Color :type "LinearColor Structure"))
  ;[1 1 1] Set Parameters
  (`MaterialInstanceDynamic.SetTextureParameterValue` `Dyn Mat Inst` "BaseColor" BaseColor)
  (`MaterialInstanceDynamic.SetTextureParameterValue` `Dyn Mat Inst` "Roughness" Roughness)
  (`MaterialInstanceDynamic.SetTextureParameterValue` `Dyn Mat Inst` "Normal" Normal)
  (`MaterialInstanceDynamic.SetVectorParameterValue` `Dyn Mat Inst` "Color" Color)
  (`MaterialInstanceDynamic.SetScalarParameterValue` `Dyn Mat Inst` "ErodeValue" 1.1))