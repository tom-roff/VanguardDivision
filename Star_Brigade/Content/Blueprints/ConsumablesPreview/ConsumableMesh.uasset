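; Preview actor that displays a selected consumable, such as walls, turrets, mines or support devices, as a spinning hologram.
; SetMeshToSelected switches on the consumable type to assign its static mesh, with per-item scale and vertical offset to frame it.
; It then overrides every material slot with an orange hologram material.
; Tick yaws the mesh a fixed step each frame, so spin speed depends on frame rate.
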(event `self.ReceiveTick`
  (params (DeltaSeconds :type "Float (single-precision)"))
  (bind _staticmesh (`self.StaticMesh`))
  (`SceneComponent.K2_SetWorldRotation` _staticmesh (`KismetMathLibrary.MakeRotator` 0.0 0.0 (+ (.yaw (`SceneComponent.K2_GetComponentRotation` _staticmesh)) 1.0)) false false))

(event `SetMeshToSelected`
  (params (Consumable :type "/Game/Blueprints/AllLevels/Variables/Enums/Consumables Enum" :default "NewEnumerator3"))
  (bind _staticmesh (`self.StaticMesh`))
  (switch `/Game/Blueprints/AllLevels/Variables/Enums/Consumables` Consumable
    (:`NewEnumerator3`
      (`StaticMeshComponent.SetStaticMesh` _staticmesh "/Game/Geometry/Meshes/Engiwall/ENGIWALL.ENGIWALL")
      (`SceneComponent.SetWorldScale3D` _staticmesh (1.0 1.0 1.0))
      (`SceneComponent.K2_SetRelativeLocation` _staticmesh (0.0 0.0 0.0) false false))
    (:`NewEnumerator4`
      (`StaticMeshComponent.SetStaticMesh` _staticmesh "/Game/Geometry/Meshes/Engiwall/Extended/ENGIWALLextended.ENGIWALLextended")
      (`SceneComponent.SetWorldScale3D` _staticmesh (0.8 0.8 0.8))
      (`SceneComponent.K2_SetRelativeLocation` _staticmesh (0.0 0.0 -50.0) false false))
    (:`NewEnumerator5`
      (`StaticMeshComponent.SetStaticMesh` _staticmesh "/Game/Geometry/Meshes/Platform/Platform.Platform")
      (`SceneComponent.SetWorldScale3D` _staticmesh (0.75 0.75 0.75))
      (`SceneComponent.K2_SetRelativeLocation` _staticmesh (0.0 0.0 0.0) false false))
    (:`NewEnumerator2`
      (`StaticMeshComponent.SetStaticMesh` _staticmesh "/Game/Geometry/Meshes/AutoTurret/AutoTurret_AutoTurretGun_.AutoTurret_AutoTurretGun_")
      (`SceneComponent.SetWorldScale3D` _staticmesh (3.5 3.5 3.5))
      (`SceneComponent.K2_SetRelativeLocation` _staticmesh (0.0 0.0 -450.0) false false))
    (:`NewEnumerator0`
      (`StaticMeshComponent.SetStaticMesh` _staticmesh "/Game/Geometry/Meshes/GrenadeTurret/GrenadeTurret.GrenadeTurret")
      (`SceneComponent.SetWorldScale3D` _staticmesh (1.0 1.0 1.0))
      (`SceneComponent.K2_SetRelativeLocation` _staticmesh (0.0 0.0 0.0) false false))
    (:`NewEnumerator6`
      (`StaticMeshComponent.SetStaticMesh` _staticmesh "/Game/Geometry/Meshes/ForceZone/ForceZone.ForceZone")
      (`SceneComponent.SetWorldScale3D` _staticmesh (1.0 1.0 1.0))
      (`SceneComponent.K2_SetRelativeLocation` _staticmesh (0.0 0.0 -50.0) false false))
    (:`NewEnumerator7`
      (`StaticMeshComponent.SetStaticMesh` _staticmesh "/Game/Geometry/Meshes/PMG/PMG.PMG")
      (`SceneComponent.SetWorldScale3D` _staticmesh (1.0 1.0 1.0))
      (`SceneComponent.K2_SetRelativeLocation` _staticmesh (0.0 0.0 0.0) false false))
    (:`NewEnumerator8`
      (`StaticMeshComponent.SetStaticMesh` _staticmesh "/Game/Geometry/Meshes/Overcharger/Overcharger.Overcharger")
      (`SceneComponent.SetWorldScale3D` _staticmesh (1.0 1.0 1.0))
      (`SceneComponent.K2_SetRelativeLocation` _staticmesh (0.0 0.0 0.0) false false))
    (:`NewEnumerator9`
      (`StaticMeshComponent.SetStaticMesh` _staticmesh "/Game/Geometry/Meshes/GaussAmplifier/GaussAmplifier.GaussAmplifier")
      (`SceneComponent.SetWorldScale3D` _staticmesh (1.0 1.0 1.0))
      (`SceneComponent.K2_SetRelativeLocation` _staticmesh (0.0 0.0 0.0) false false))
    (:`NewEnumerator10`
      (`StaticMeshComponent.SetStaticMesh` _staticmesh "/Game/Geometry/Meshes/ProxMine/ProxMine.ProxMine")
      (`SceneComponent.SetWorldScale3D` _staticmesh (1.0 1.0 1.0))
      (`SceneComponent.K2_SetRelativeLocation` _staticmesh (0.0 0.0 0.0) false false)))
  (for _index (range (+ (`PrimitiveComponent.GetNumMaterials` (`self.StaticMesh`)) 1))
    (`PrimitiveComponent.SetMaterial` _staticmesh _index "/Game/Materials/HologramMat/HologramOrange.HologramOrange")))

(fn `UserConstructionScript`)