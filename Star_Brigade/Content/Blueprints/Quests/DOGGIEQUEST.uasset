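; Quest actor that tracks the dog quest through a Stage value: Beginning, Dog Helped and Quest Completed.
; StartQuest sets the first stage, finds the first DOGGIE actor in the level and calls its DogQuestStart.
; The DogHelped and TalkToOwner events advance the stage, with TalkToOwner completing the quest.
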(event `StartQuest`
  (set `self.Stage` "Beginning")
  (bind _outactors (`GameplayStatics.GetAllActorsOfClass` "/Game/Blueprints/DOGGIE.DOGGIE_C"))
  (`/Game/Blueprints/DOGGIE.DogQuestStart` (`|GetArrayItem` _outactors)))

(event `DogHelped`
  (set `self.Stage` "Dog Helped"))

(event `TalkToOwner`
  (set `self.Stage` "Quest Completed"))

(fn `UserConstructionScript`
  (`parent.UserConstructionScript`))