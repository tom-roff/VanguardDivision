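; Jump pad level object that launches any Character entering its Overlap component.
; On overlap it stops the character's movement, then calls LaunchCharacter with overrides on all axes.
; The launch velocity combines the Arrow component's forward direction scaled by a horizontal strength with a separate vertical strength.
; An emitter spawns at the Overlap component's location on each launch.
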(event `self.Overlap.OnComponentBeginOverlap`
  (params (OverlappedComponent :type "PrimitiveComponent Object Reference") (OtherActor :type "Actor Object Reference") (OtherComp :type "PrimitiveComponent Object Reference") (OtherBodyIndex :type Integer) (bFromSweep :type Boolean) (SweepResult :type "HitResult Structure (by ref)"))
  (bind _ascharacter (cast `Character` OtherActor))
  (`MovementComponent.StopMovementImmediately` (`Character.CharacterMovement` _ascharacter))
  (`Character.LaunchCharacter` _ascharacter (+ (* (`SceneComponent.GetForwardVector` (`self.Arrow`)) (`self.Horizontal Strength`)) (`KismetMathLibrary.MakeVector` 0.0 0.0 (`self.Vertical Strength`))) true true)
  (`GameplayStatics.SpawnEmitterAtLocation` null (`SceneComponent.K2_GetComponentLocation` (`self.Overlap`))))

(fn `UserConstructionScript`)