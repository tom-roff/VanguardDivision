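; KillBox is a level object that kills the player and enemies that overlap it.
; On overlap, it casts the other actor to TrueFirstPersonCharacter and calls PlayerDie with that character's player controller.
; Otherwise, actors whose class derives from EnemyParent receive a huge ApplyDamage hit, with the box as damage causer.
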(event `self.ReceiveActorBeginOverlap`
  (params (OtherActor :type "Actor Object Reference"))
  (bind _astrue_first_person_character (cast `/Game/TrueFPP/TrueFirstPersonCharacter` OtherActor)
    (:`then`
      (`/Game/TrueFPP/TrueFirstPersonCharacter.PlayerDie` _astrue_first_person_character (cast `PlayerController` (`Pawn.GetController` _astrue_first_person_character) :!pure true)))
    (:`CastFailed`
      (if (`KismetMathLibrary.ClassIsChildOf` (`GameplayStatics.GetObjectClass` OtherActor) "/Game/Blueprints/AIActorsPawns/EnemyParent.EnemyParent_C")
        (`GameplayStatics.ApplyDamage` OtherActor 99999.0 null self)))))

(fn `UserConstructionScript`)