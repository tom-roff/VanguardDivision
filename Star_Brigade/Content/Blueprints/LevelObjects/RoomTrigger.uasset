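; RoomTrigger is a level volume that tracks whether player characters occupy a room and reports it to the wave game mode.
; On the server, a TrueFirstPersonCharacter entering sets IsOpen and adds the trigger uniquely to WaveGMUpdated's ActiveRooms.
; When the last overlapping character leaves, the server removes the trigger from that list; IsOpen is never reset here.
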(event `TellServerOverlap`
  ;[1 1 1] When a player character enters, tell server that the zone is active.
  (bind _aswave_gmupdated (cast `/Game/Blueprints/Gameplay/WaveGMUpdated` (`GameplayStatics.GetGameMode`)))
  (`KismetArrayLibrary.Array_AddUnique` (`/Game/Blueprints/Gameplay/WaveGMUpdated.ActiveRooms` _aswave_gmupdated) self))

(event `self.ReceiveActorBeginOverlap`
  (params (OtherActor :type "Actor Object Reference"))
  ;[1 1 1] When a player character enters, tell server that the zone is active.
  (if (== (`GameplayStatics.GetObjectClass` OtherActor) "/Game/TrueFPP/TrueFirstPersonCharacter.TrueFirstPersonCharacter_C")
    (`/Engine/EditorBlueprintResources/ActorMacros.Switch Has Authority`
      (:`Authority`
        (set `self.IsOpen?` true)
        (`self.TellServerOverlap`)))))

(event `self.ReceiveActorEndOverlap`
  (params (OtherActor :type "Actor Object Reference"))
  ;[1 1 1] When all players have left, server says area is no longer active
  (if (== (`GameplayStatics.GetObjectClass` OtherActor) "/Game/TrueFPP/TrueFirstPersonCharacter.TrueFirstPersonCharacter_C")
    (if (not (`KismetArrayLibrary.Array_IsValidIndex` (`PrimitiveComponent.GetOverlappingActors` (`self.Trigger`) "/Game/TrueFPP/TrueFirstPersonCharacter.TrueFirstPersonCharacter_C")))
      (`/Engine/EditorBlueprintResources/ActorMacros.Switch Has Authority`
        (:`Authority`
          (`self.TellServerStopOverlap`))))))

(event `TellServerStopOverlap`
  ;[1 1 1] When all players have left, server says area is no longer active
  (bind _aswave_gmupdated (cast `/Game/Blueprints/Gameplay/WaveGMUpdated` (`GameplayStatics.GetGameMode`)))
  (`KismetArrayLibrary.Array_RemoveItem` (`/Game/Blueprints/Gameplay/WaveGMUpdated.ActiveRooms` _aswave_gmupdated) self))

(fn `UserConstructionScript`)