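; Game instance that serves as the central hub for audio settings, menus, saving and Steam multiplayer sessions across all levels.
; It applies saved volumes through sound mix overrides, creates menu, loading, fade and error widgets, and tracks weapon ammo.
; Player, story and weapon data save to separate slots via load-or-create events.
; Advanced Sessions nodes host listen-server lobbies and join sessions or invites, saving and destroying the current session first.
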(event `ChangeMasterVolume`
  (params (AudioVolume :type "Float (double-precision)"))
  ;[1 1 1] Audio System
  ;;[1 1 1] Change Different Volumes
  (set `self.MasterVolume` AudioVolume)
  (`GameplayStatics.SetSoundMixClassOverride` "/Game/Audio/BaseSoundMix.BaseSoundMix" "/Game/Audio/MasterSoundClass.MasterSoundClass" (`KismetMathLibrary.FClamp` (`self.MasterVolume`)) 1.0 0.0))

(event `self.ReceiveInit`
  ;[1 1 1] Audio System
  ;;[1 1 1] On Game Initialize, set the base sound mix
  (`KismetSystemLibrary.Delay` 0.1)
  (`GameplayStatics.SetBaseSoundMix` "/Game/Audio/BaseSoundMix.BaseSoundMix")
  (`self.SetAudioSettings`))

(event `ChangeAmbienceVolume`
  (params (AudioVolume :type "Float (double-precision)"))
  ;[1 1 1] Audio System
  ;;[1 1 1] Change Different Volumes
  (set `self.AmbienceVolume` AudioVolume)
  (`GameplayStatics.SetSoundMixClassOverride` "/Game/Audio/BaseSoundMix.BaseSoundMix" "/Game/Audio/Ambience.Ambience" (`KismetMathLibrary.FClamp` (`self.AmbienceVolume`)) 1.0 0.0))

(event `SetAudioSettings`
  ;[1 1 1] Audio System
  ;;[1 1 1] Audio Settings Saving
  (bind _returnvalue (`GameplayStatics.LoadGameFromSlot` "Settings"))
  (bind _asplayer_settings_save (cast `/Game/Blueprints/AllLevels/SaveGames/PlayerSettingsSave` _returnvalue))
  (bind (_mastervolume _musicvolume _ambiencevolume _soundeffectsvolume _audioquality) (break `/Game/Blueprints/AllLevels/Variables/Structs/UserAudioSettings` (`/Game/Blueprints/AllLevels/SaveGames/PlayerSettingsSave.UserAudioSettings` _asplayer_settings_save)))
  (`self.ChangeMasterVolume` _mastervolume)
  (`self.ChangeAmbienceVolume` _ambiencevolume)
  (`self.ChangeMusicVolume` _musicvolume)
  (`self.ChangeSoundEffectsVolume` _soundeffectsvolume)
  (bind _returnvalue_2 (`GameUserSettings.GetGameUserSettings`))
  (`GameUserSettings.SetAudioQualityLevel` _returnvalue_2 _audioquality))

(event `ChangeMusicVolume`
  (params (AudioVolume :type "Float (double-precision)"))
  ;[1 1 1] Audio System
  ;;[1 1 1] Change Different Volumes
  (set `self.MusicVolume` AudioVolume)
  (`GameplayStatics.SetSoundMixClassOverride` "/Game/Audio/BaseSoundMix.BaseSoundMix" "/Game/Audio/Music.Music" (`KismetMathLibrary.FClamp` (`self.MusicVolume`)) 1.0 0.0))

(event `ChangeSoundEffectsVolume`
  (params (AudioVolume :type "Float (double-precision)"))
  ;[1 1 1] Audio System
  ;;[1 1 1] Change Different Volumes
  (set `self.SoundEffectsVolume` AudioVolume)
  (`GameplayStatics.SetSoundMixClassOverride` "/Game/Audio/BaseSoundMix.BaseSoundMix" "/Game/Audio/SoundEffects.SoundEffects" (`KismetMathLibrary.FClamp` (`self.SoundEffectsVolume`)) 1.0 0.0))

(event `ShowMainMenu`
  ;[1 1 1] UI Management
  ;;[1 1 1] Show Main Menu and Mouse Cursor
  (`/Engine/EditorBlueprintResources/StandardMacros.IsValid` (`self.MainMenuWB`)
    (:`Is Valid`
      _)
    (:`Is Not Valid`
      (bind _returnvalue (`|CreateWidget` "/Game/UI_elements/Menus/MainMenu/MainMenu.MainMenu_C" (`GameplayStatics.GetPlayerController` 0)))
      (set `self.MainMenuWB` _returnvalue)))
  (`UserWidget.AddToViewport` (`self.MainMenuWB`) 0)
  (set `PlayerController.bShowMouseCursor` true (`GameplayStatics.GetPlayerController` 0)))

(event `self.HandleNetworkError`
  (params (FailureType :type "ENetworkFailure Enum" :default "NetDriverAlreadyExists") (bIsServer :type Boolean))
  ;[1 1 1] Errors
  ;;[1 1 1] Handle Network Errors and Tell That Something's Wrong
  (`self.ShowErrorMessage` FailureType "Network Error"))

(event `SaveStoryPostAck`
  (params (`Save Game` :type "SaveGame Object Reference"))
  ;[1 1 1] Saving and Game Logic
  ;;[1 1 1] Save Story Progress when called (called in Save Game event too, so no need for extra event adding)
  (bind _asplayer_controller_main (cast `/Game/Blueprints/AllLevels/PlayerControllerMain` (`GameplayStatics.GetPlayerController` 0)))
  (bind _asplayer_story_save (cast `/Game/Blueprints/AllLevels/SaveGames/PlayerStorySave` `Save Game`))
  (set `/Game/Blueprints/AllLevels/SaveGames/PlayerStorySave.S_PlayerStoryInfo` (`/Game/Blueprints/AllLevels/PlayerControllerMain.PlayerStoryInfoController` _asplayer_controller_main) _asplayer_story_save)
  (`GameplayStatics.SaveGameToSlot` `Save Game` "Story"))

(event `Save Story`
  ;[1 1 1] Saving and Game Logic
  ;;[1 1 1] Save Story Progress when called (called in Save Game event too, so no need for extra event adding)
  (bind _returnvalue (`GameplayStatics.DoesSaveGameExist` "Story"))
  (if _returnvalue
    (bind _returnvalue_2 (`GameplayStatics.LoadGameFromSlot` "Story"))
    (`self.SaveStoryPostAck` _returnvalue_2)
    (else
      (bind _returnvalue_3 (`GameplayStatics.CreateSaveGameObject` "/Game/Blueprints/AllLevels/SaveGames/PlayerStorySave.PlayerStorySave_C"))
      (`self.SaveStoryPostAck` _returnvalue_3))))

(event `SetWeaponAmmos`
  ;[1 1 1] Saving and Game Logic
  ;;[1 1 1] Set Weapon Ammo
  (bind _astrue_first_person_character (cast `/Game/TrueFPP/TrueFirstPersonCharacter` (`GameplayStatics.GetPlayerCharacter` 0)))
  (bind _currentweaponinhand (`/Game/TrueFPP/TrueFirstPersonCharacter.CurrentWeaponInHand` _astrue_first_person_character))
  (bind _asgun_parent (cast `/Game/Blueprints/Weapons/GunParent` _currentweaponinhand))
  (bind _returnvalue (`GameplayStatics.GetObjectClass` _currentweaponinhand))
  (bind (_equippedwep1new _class _equippedweapon2) (break `/Game/Blueprints/AllLevels/Variables/Structs/PlayerInfoBase` (`/Game/TrueFPP/TrueFirstPersonCharacter.PlayerInfo` _astrue_first_person_character)))
  (if (== _returnvalue _equippedwep1new)
    (bind _currentammototal (`/Game/Blueprints/Weapons/GunParent.CurrentAmmoTotal` _asgun_parent))
    (set `self.Weapon1AmmoTotal` _currentammototal)
    (bind _currentammoinmag (`/Game/Blueprints/Weapons/GunParent.CurrentAmmoInMag` _asgun_parent))
    (set `self.Weapon1AmmoInMag` _currentammoinmag)
    (elif (== _returnvalue _equippedweapon2)
      (set `self.Weapon2AmmoTotal` _currentammototal)
      (set `self.Weapon2AmmoInMag` _currentammoinmag)
      (else
        (set `self.Weapon3AmmoTotal` _currentammototal)
        (set `self.Weapon3AmmoInMag` _currentammoinmag)))))

(event `ShowServerMenu`
  ;[1 1 1] UI Management
  ;;[1 1 1] Shows Server Menu
  (bind _returnvalue (`|CreateWidget` "/Game/UI_elements/Menus/MainMenu/Multiplayer/ServerMenu.ServerMenu_C" (`GameplayStatics.GetPlayerController` 0)))
  (`UserWidget.AddToViewport` _returnvalue 0))

(event `ShowOptionsMenu`
  ;[1 1 1] UI Management
  ;;[1 1 1] Shows Options Menu
  (`/Engine/EditorBlueprintResources/StandardMacros.IsValid` (`self.SettingsMenuWB`)
    (:`Is Valid`
      _)
    (:`Is Not Valid`
      (bind _returnvalue (`|CreateWidget` "/Game/UI_elements/PauseMenu/PauseOptions.PauseOptions_C" (`GameplayStatics.GetPlayerController` 0)))
      (bind _output_get (set `self.SettingsMenuWB` _returnvalue))))
  (`UserWidget.AddToViewport` _output_get 0))

(event `self.HandleTravelError`
  (params (FailureType :type "ETravelFailure Enum" :default "NoLevel"))
  ;[1 1 1] Errors
  ;;[1 1 1] Handle Travel Errors and Tell That Something's Wrong
  (`self.ShowErrorMessage` "NetDriverAlreadyExists" "Error Traveling " true FailureType))

(event `JoinServer`
  (params (SessionToJoin :type "BlueprintSessionResult Structure"))
  ;[1 1 1] UI Management
  ;;[1 1 1] Join Server
  (`self.ShowLoadingScreen`)
  (`JoinSessionCallbackProxy.JoinSession` (`GameplayStatics.GetPlayerController` 0) SessionToJoin
    (:`OnFailure`
      (`self.ShowErrorMessage` "ConnectionLost" "Failed to join game session." false "ClientTravelFailure"))))

(event `ShowLoadingScreen`
  ;[1 1 1] UI Management
  ;;[1 1 1] Shows Loading Screen
  (`/Engine/EditorBlueprintResources/StandardMacros.IsValid` (`self.LoadingWB`)
    (:`Is Valid`
      _)
    (:`Is Not Valid`
      (bind _returnvalue (`|CreateWidget` "/Game/UI_elements/Menus/Loading.Loading_C" (`GameplayStatics.GetPlayerController` 0)))
      (bind _output_get (set `self.LoadingWB` _returnvalue))))
  (`UserWidget.AddToViewport` _output_get 0))

(event `ShowErrorMessage`
  (params (ErrorType :type "ENetworkFailure Enum" :default "NetDriverAlreadyExists") (TextToShow :type Text) (`IsTravelError?` :type Boolean) (TravelErrorType :type "ETravelFailure Enum" :default "NoLevel"))
  ;[1 1 1] Errors
  ;;[1 1 1] Show Error Message
  (`KismetSystemLibrary.Delay` 1.0)
  (`/Engine/EditorBlueprintResources/StandardMacros.IsValid` (stale _returnvalue)
    (:`Is Valid`
      _)
    (:`Is Not Valid`
      (bind _returnvalue (`|CreateWidget` "/Game/UI_elements/Menus/MainMenu/ErrorMessageWB.ErrorMessageWB_C" (`GameplayStatics.GetPlayerController` 0)))))
  (set `/Game/UI_elements/Menus/MainMenu/ErrorMessageWB.ErrorTextToShow` TextToShow _returnvalue)
  (set `/Game/UI_elements/Menus/MainMenu/ErrorMessageWB.ErrorType` ErrorType _returnvalue)
  (set `/Game/UI_elements/Menus/MainMenu/ErrorMessageWB.IsTravelError?` `IsTravelError?` _returnvalue)
  (set `/Game/UI_elements/Menus/MainMenu/ErrorMessageWB.TravelErrorType` TravelErrorType _returnvalue)
  (`UserWidget.AddToViewport` _returnvalue 10))

(event `SaveGamePostSaveAcknowledgement`
  (params (SaveGameRef :type "SaveGame Object Reference"))
  (bind _returnvalue (`GameplayStatics.GetPlayerController` 0))
  (bind _basesaveref (`self.BaseSaveRef`))
  ;[1 1 1] Saving and Game Logic
  ;;[1 1 1] Save Game to Slot when called
  (bind _asplayer_save_game (cast `/Game/Blueprints/AllLevels/SaveGames/PlayerSaveGame` SaveGameRef))
  (set `self.BaseSaveRef` _asplayer_save_game)
  (bind _astrue_first_person_character (cast `/Game/TrueFPP/TrueFirstPersonCharacter` (`GameplayStatics.GetPlayerCharacter` 0)))
  (set `/Game/Blueprints/AllLevels/SaveGames/PlayerSaveGame.S_PlayerInfoBase` (`/Game/TrueFPP/TrueFirstPersonCharacter.PlayerInfo` _astrue_first_person_character) _basesaveref)
  (set `/Game/Blueprints/AllLevels/SaveGames/PlayerSaveGame.CurrentLevel` (`/Game/TrueFPP/TrueFirstPersonCharacter.CurrentLevel` _astrue_first_person_character) _basesaveref)
  (set `/Game/Blueprints/AllLevels/SaveGames/PlayerSaveGame.PrevReqdLvlUpXP` (`/Game/TrueFPP/TrueFirstPersonCharacter.PreviousReqdLvlUpXP` _astrue_first_person_character) _basesaveref)
  (bind _returnvalue_2 (`GameplayStatics.SaveGameToSlot` (`self.BaseSaveRef`) "1"))
  (if _returnvalue_2
    (`/Engine/EditorBlueprintResources/StandardMacros.IsValid` (stale _returnvalue_3)
      (:`Is Valid`
        _)
      (:`Is Not Valid`
        (bind _returnvalue_3 (`|CreateWidget` "/Game/UI_elements/Notifications/GameSaved.GameSaved_C" _returnvalue))))
    (`UserWidget.AddToViewport` _returnvalue_3 0)
    (set `/Game/UI_elements/Notifications/GameSaved.TextToShow` "Game Saved" _returnvalue_3)
    (`self.RemoveSaveWBInst` _returnvalue_3)
    (else
      (`/Engine/EditorBlueprintResources/StandardMacros.IsValid` (stale _returnvalue_4)
        (:`Is Valid`
          _)
        (:`Is Not Valid`
          (bind _returnvalue_4 (`|CreateWidget` "/Game/UI_elements/Notifications/GameSaved.GameSaved_C" _returnvalue))))
      (`UserWidget.AddToViewport` _returnvalue_4 0)
      (set `/Game/UI_elements/Notifications/GameSaved.TextToShow` "Save Failed" _returnvalue_4)
      (`self.RemoveSaveWBInst` _returnvalue_4))))

(event `Save Game Event`
  ;[1 1 1] Saving and Game Logic
  ;;[1 1 1] Save Game to Slot when called
  (`self.Save Weapons`)
  (bind _returnvalue (`GameplayStatics.DoesSaveGameExist` "1"))
  (if _returnvalue
    (bind _returnvalue_2 (`GameplayStatics.LoadGameFromSlot` "1"))
    (`self.SaveGamePostSaveAcknowledgement` _returnvalue_2)
    (else
      (bind _returnvalue_3 (`GameplayStatics.CreateSaveGameObject` "/Game/Blueprints/AllLevels/SaveGames/PlayerSaveGame.PlayerSaveGame_C"))
      (`self.SaveGamePostSaveAcknowledgement` _returnvalue_3))))

(event `RemoveSaveWBInst`
  (params (Target :type "/Game/UI_elements/Notifications/GameSaved Object Reference"))
  ;[1 1 1] Saving and Game Logic
  ;;[1 1 1] Save Game to Slot when called
  (`KismetSystemLibrary.Delay` 1.4)
  (`/Engine/EditorBlueprintResources/StandardMacros.IsValid` Target
    (:`Is Valid`
      (`/Game/UI_elements/Notifications/GameSaved.RemoveSaveWB` Target))))

(event `FadeOutOfBlack`
  (params (`Fade Out Duration` :type "Float (double-precision)"))
  ;[1 1 1] Fade in and out of black
  (bind _foundwidgets (`WidgetBlueprintLibrary.GetAllWidgetsOfClass` "/Game/UI_elements/BlackScreen.BlackScreen_C" false))
  (for _array_element _foundwidgets
    (`/Engine/EditorBlueprintResources/StandardMacros.IsValid` _array_element
      (:`Is Valid`
        (`/Game/UI_elements/BlackScreen.FadeOutOfBlack` _array_element `Fade Out Duration`)))))

(event `FadeToBlack`
  (params (`Fade In Duration` :type "Float (double-precision)"))
  ;[1 1 1] Fade in and out of black
  (`/Engine/EditorBlueprintResources/StandardMacros.IsValid` (stale _returnvalue)
    (:`Is Valid`
      _)
    (:`Is Not Valid`
      (bind _returnvalue (`|CreateWidget` "/Game/UI_elements/BlackScreen.BlackScreen_C" (`GameplayStatics.GetPlayerController` 0)))))
  (if (not (`Widget.IsInViewport` _returnvalue))
    (`UserWidget.AddToViewport` _returnvalue 0))
  (`/Game/UI_elements/BlackScreen.Fade to Black` _returnvalue `Fade In Duration`))

(event `SaveWepsPostAck`
  (params (SaveGameRef :type "SaveGame Object Reference"))
  ;[1 1 1] Saving and Game Logic
  ;;[1 1 1] Player Weapons Saving
  (bind _asplayer_weapons_save (cast `/Game/Blueprints/AllLevels/SaveGames/PlayerWeaponsSave` SaveGameRef))
  (bind _astrue_first_person_character (cast `/Game/TrueFPP/TrueFirstPersonCharacter` (`GameplayStatics.GetPlayerCharacter` 0)))
  (set `/Game/Blueprints/AllLevels/SaveGames/PlayerWeaponsSave.S_PlayerWeapons` (`/Game/TrueFPP/TrueFirstPersonCharacter.PlayerWeaponsInfo` _astrue_first_person_character) _asplayer_weapons_save)
  (`GameplayStatics.SaveGameToSlot` _asplayer_weapons_save "Weapons"))

(event `Save Weapons`
  ;[1 1 1] Saving and Game Logic
  ;;[1 1 1] Player Weapons Saving
  (bind _returnvalue (`GameplayStatics.DoesSaveGameExist` "Weapons"))
  (if _returnvalue
    (bind _returnvalue_2 (`GameplayStatics.LoadGameFromSlot` "Weapons"))
    (`self.SaveWepsPostAck` _returnvalue_2)
    (else
      (bind _returnvalue_3 (`GameplayStatics.CreateSaveGameObject` "/Game/Blueprints/AllLevels/SaveGames/PlayerWeaponsSave.PlayerWeaponsSave_C"))
      (`self.SaveWepsPostAck` _returnvalue_3))))

(event `self.OnSessionInviteAccepted`
  (params (LocalPlayerNum :type Integer) (PersonInvited :type "BPUniqueNetId Structure") (SessionToJoin :type "BlueprintSessionResult Structure (by ref)"))
  (bind _returnvalue (`GameplayStatics.GetPlayerController` 0))
  (bind _returnvalue_2 (`GameplayStatics.GetPlayerController` 0))
  (bind _sessiontojoin (`self.SessionToJoin`))
  ;[1 1 1] Multiplayer Connections
  ;;[1 1 1] When Invite is Accepted, join the session
  (set `self.SessionToJoin` SessionToJoin)
  (`self.Save Game Event`)
  (bind _returnvalue_3 (`|CreateWidget` "/Game/UI_elements/Menus/Loading.Loading_C" _returnvalue_2))
  (`WidgetBlueprintLibrary.SetInputMode_UIOnlyEx` _returnvalue_2 null)
  (`UserWidget.AddToViewport` _returnvalue_3 0)
  (`DestroySessionCallbackProxy.DestroySession` (`GameplayStatics.GetPlayerController` 0)
    (:`OnSuccess`
      _)
    (:`OnFailure`
      _))
  (if (< (`FindSessionsCallbackProxy.GetCurrentPlayers` _sessiontojoin) (`FindSessionsCallbackProxy.GetMaxPlayers` _sessiontojoin))
    (`JoinSessionCallbackProxy.JoinSession` _returnvalue _sessiontojoin
      (:`OnSuccess`
        (`WidgetBlueprintLibrary.SetInputMode_GameOnly` _returnvalue))
      (:`OnFailure`
        (`self.ShowErrorMessage` "ConnectionLost" "Failed to join game session.")))
    (else
      (`self.ShowErrorMessage` "FailureReceived" "The game is full."))))

(event `SetWeaponAmmosToMax`
  ;[1 1 1] Saving and Game Logic
  ;;[1 1 1] Set Player Weapons to Max When Called
  (bind _astrue_first_person_character (cast `/Game/TrueFPP/TrueFirstPersonCharacter` (`GameplayStatics.GetPlayerCharacter` 0)))
  (bind (_equippedwep1new _class _equippedweapon2 _equippedtool) (break `/Game/Blueprints/AllLevels/Variables/Structs/PlayerInfoBase` (`/Game/TrueFPP/TrueFirstPersonCharacter.PlayerInfo` _astrue_first_person_character)))
  (bind _asgun_parent (castclass `/Game/Blueprints/Weapons/GunParent` _equippedwep1new)) ; Weapon 1 Ammo Setting
  (bind (_damage _firerate _reloadspeed _maxammototal _maxammopermag) (break `/Game/Blueprints/Weapons/WeaponStats` (`.WeaponStats` (defaults `Object` _asgun_parent))))
  (set `self.Weapon1AmmoInMag` _maxammopermag)
  (set `self.Weapon1AmmoTotal` _maxammototal)
  (bind _asgun_parent_2 (castclass `/Game/Blueprints/Weapons/GunParent` _equippedweapon2))
  (bind (_damage_2 _firerate_2 _reloadspeed_2 _maxammototal_2 _maxammopermag_2) (break `/Game/Blueprints/Weapons/WeaponStats` (`.WeaponStats` (defaults `Object` _asgun_parent_2))))
  (set `self.Weapon2AmmoInMag` _maxammopermag_2)
  (set `self.Weapon2AmmoTotal` _maxammototal_2)
  (bind _asgun_parent_3 (castclass `/Game/Blueprints/Weapons/GunParent` _equippedtool))
  (bind (_damage_3 _firerate_3 _reloadspeed_3 _maxammototal_3 _maxammopermag_3) (break `/Game/Blueprints/Weapons/WeaponStats` (`.WeaponStats` (defaults `Object` _asgun_parent_3))))
  (set `self.Weapon3AmmoTotal` _maxammototal_3)
  (set `self.Weapon3AmmoInMag` _maxammopermag_3)
  (`/Game/TrueFPP/TrueFirstPersonCharacter.EquipGun1` _astrue_first_person_character))

(event `ShowHostMenu`
  ;[1 1 1] Multiplayer Connections
  ;;[1 1 1] Host Game Menu
  (`/Engine/EditorBlueprintResources/StandardMacros.IsValid` (`self.HostMenuWB`)
    (:`Is Valid`
      _)
    (:`Is Not Valid`
      (bind _returnvalue (`|CreateWidget` "/Game/UI_elements/Menus/MainMenu/Multiplayer/HostMenu.HostMenu_C" (`GameplayStatics.GetPlayerController` 0)))
      (bind _output_get (set `self.HostMenuWB` _returnvalue))))
  (`UserWidget.AddToViewport` _output_get 0))

(event `JoinSessionEvent`
  (params (Result :type "BlueprintSessionResult Structure (by ref)"))
  (bind _returnvalue (`GameplayStatics.GetPlayerController` 0))
  (bind _returnvalue_2 (`GameplayStatics.GetPlayerController` 0))
  ;[1 1 1] Multiplayer Connections
  ;;[1 1 1] When Invite is Accepted, join the session
  (`KismetSystemLibrary.PrintString` (`AdvancedSessionsLibrary.GetSessionID_AsString` Result))
  (`self.Save Game Event`)
  (bind _returnvalue_3 (`|CreateWidget` "/Game/UI_elements/Menus/Loading.Loading_C" _returnvalue))
  (`WidgetBlueprintLibrary.SetInputMode_UIOnlyEx` _returnvalue null)
  (`UserWidget.AddToViewport` _returnvalue_3 0)
  (`DestroySessionCallbackProxy.DestroySession` (`GameplayStatics.GetPlayerController` 0)
    (:`OnSuccess`
      _)
    (:`OnFailure`
      _))
  (`JoinSessionCallbackProxy.JoinSession` _returnvalue_2 Result
    (:`OnSuccess`
      (`WidgetBlueprintLibrary.SetInputMode_GameOnly` _returnvalue_2))
    (:`OnFailure`
      (`self.ShowErrorMessage` "ConnectionLost" "Failed to join game session."))))

(event `LaunchLobby`
  (params (`EnableLan?` :type Boolean) (LevelToOpen :type Name))
  ;[1 1 1] Multiplayer Connections
  ;;[1 1 1] Launch Lobby
  (`self.ShowLoadingScreen`)
  (`CreateSessionCallbackProxyAdvanced.CreateAdvancedSession` (`|MakeArray` (`AdvancedSessionsLibrary.MakeLiteralSessionPropertyString` "UniqueID" (`AdvancedSessionsLibrary.GetCurrentSessionID_AsString`))) (`GameplayStatics.GetPlayerController` 0) 4 0 `EnableLan?` true false true true true true true
    (:`OnSuccess`
      (`GameplayStatics.OpenLevel` LevelToOpen true "listen"))
    (:`OnFailure`
      (`self.ShowErrorMessage` "ConnectionLost" "Failed to Create Steam Session.  "))))

(event `DestroySessionCaller`
  (params (PlayerController :type "PlayerController Object Reference"))
  ;[1 1 1] Multiplayer Connections
  ;;[1 1 1] Destroy Session
  (`DestroySessionCallbackProxy.DestroySession` PlayerController
    (:`OnFailure`
      (`self.ShowErrorMessage` "FailureReceived" "Failed to Destroy Session."))))

(event `SetNameAndPicture`
  (bind _returnvalue (`GameplayStatics.GetPlayerController` 0))
  ;[1 1 1] Multiplayer Connections
  ;;[1 1 1] Set in game name and picture according to Steam
  (set `self.SteamName` (`AdvancedSessionsLibrary.GetPlayerName` _returnvalue))
  (bind _returnvalue_2 (`AdvancedSteamFriendsLibrary.GetSteamFriendAvatar` (`AdvancedSessionsLibrary.GetUniqueNetID` _returnvalue) "SteamAvatar_Small")
    (:`OnSuccess`
      (set `self.PlayerSteamPicture` _returnvalue_2))
    (:`OnFailure`
      (`KismetSystemLibrary.PrintString` "Failed to retrieve steam photo"))))