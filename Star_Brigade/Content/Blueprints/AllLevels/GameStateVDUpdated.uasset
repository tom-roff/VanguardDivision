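; Game state for a multiplayer wave game, handling lobby-to-map travel, between-wave countdowns and a connected-player list.
; A looping one-second timer counts down to the game mode's StartNextWave, then resets ready state.
; StartWaveMode saves difficulty and player count to the game instance, clears readiness, then runs ServerTravel to the selected map.
; It also hosts actor visibility helpers and barrel explosions, which hide the barrel before delayed authority-only destruction.
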(event `SetBarsVis`
  (params (Target2 :type "PrimitiveComponent Object Reference"))
  (`SceneComponent.SetHiddenInGame` Target2 true false)
  (`PrimitiveComponent.SetCollisionEnabled` Target2 "NoCollision"))

(event `SetPlayerDatas`
  ;[1 1 1] SetThePlayerDatasArrayToWhateverTheThingBe
  (bind _outactors (`GameplayStatics.GetAllActorsOfClass` "/Game/Blueprints/AllLevels/PlayerControllerMain.PlayerControllerMain_C"))
  (for _array_element _outactors
    (`self.RegisterLoginGameState` (`Controller.PlayerState` _array_element))))

(event `self.ReceiveBeginPlay`
  ;[1 1 1] SetThePlayerDatasArrayToWhateverTheThingBe
)

(event `SetActorInvisible`
  (params (ActorToSetInvis :type "Actor Object Reference"))
  ;[1 1 1] Enable/Disable the Visibility of an Actor
  (`self.SetActorHiddenInGame` ActorToSetInvis true)
  (`self.SetActorEnableCollision` ActorToSetInvis false))

(event `BlowUpBarrel`
  (params (BarrelToKill :type "Actor Object Reference"))
  (bind _returnvalue (`self.K2_GetActorLocation` BarrelToKill))
  ;[1 1 1] Blow Up Barrels
  (`GameplayStatics.ApplyRadialDamage` :`BaseDamage` 60.0 :`Origin` (`self.K2_GetActorLocation` BarrelToKill) :`DamageRadius` 1000.0 :`DamageTypeClass` "/Game/Blueprints/Gameplay/ExplosiveDamageType.ExplosiveDamageType_C" :`DamageCauser` BarrelToKill :`InstigatedByController` null)
  (`GameplayStatics.PlaySoundAtLocation` "/Game/Particles/VFX_Toolkit_V1/Sounds/S_Explode_Reverb_01.S_Explode_Reverb_01" _returnvalue (struct) 1.0 1.0 0.0 "/Game/Audio/Attenuations/BaseAtten.BaseAtten" null null)
  (`GameplayStatics.SpawnEmitterAtLocation` "/Game/Particles/VFX_Toolkit_V1/ParticleSystems/356Days/Par_Meteora_Explode_01.Par_Meteora_Explode_01" _returnvalue)
  (`self.SetActorInvisible` BarrelToKill)
  (`GameplayStatics.PlayWorldCameraShake` "/Game/Blueprints/CameraShakes/ExplosionShake.ExplosionShake_C" _returnvalue 0.0 1000.0)
  (`KismetSystemLibrary.Delay` 5.0)
  (`/Engine/EditorBlueprintResources/ActorMacros.Switch Has Authority`
    (:`Authority`
      (`self.K2_DestroyActor` BarrelToKill))))

(event `SetActorVisible`
  (params (ActorToSetVis :type "Actor Object Reference"))
  ;[1 1 1] Enable/Disable the Visibility of an Actor
  (`self.SetActorHiddenInGame` ActorToSetVis false)
  (`self.SetActorEnableCollision` ActorToSetVis true))

(event `UpdateCurrentWave`
  (params (CurrentWave :type Integer))
  ;[1 1 1] Start/Stop Wave Timer, Update Current Wave
  (set `self.CurrentWave` CurrentWave))

(event `StartWaveStartTimer`
  ;[1 1 1] Start/Stop Wave Timer, Update Current Wave
  (set `self.IsAnyPlayerReady?` true)
  (set `self.NextWaveCountdownTime` (`self.DefaultNextWaveCountdownTime`))
  (bind _returnvalue (`KismetSystemLibrary.K2_SetTimerDelegate` (delegate `DecreaseCountdownTime`) 1.0 true))
  (set `self.WaveStartCountdown` _returnvalue))

(event `RegisterLoginGameState`
  (params (`New Player State` :type "PlayerState Object Reference"))
  ;[1 1 1] Party List Information
  ;;[1 1 1] When someone logs in, add their playerstate to the array
  (bind _asplayer_state_1main (cast `/Game/Blueprints/AllLevels/PlayerState1Main` `New Player State`))
  (`KismetArrayLibrary.Array_AddUnique` (`self.ConnectedPlayersGS`) _asplayer_state_1main))

(event `DecreaseCountdownTime`
  ;[1 1 1] Start/Stop Wave Timer, Update Current Wave
  (bind _output_get (set `self.NextWaveCountdownTime` (- (`self.NextWaveCountdownTime`) 1)))
  (if (== _output_get 0)
    (`self.AllPlayersReadyStartWave`)))

(event `StopWaveStartTimer`
  ;[1 1 1] Start/Stop Wave Timer, Update Current Wave
  (set `self.IsAnyPlayerReady?` false)
  (`KismetSystemLibrary.K2_ClearAndInvalidateTimerHandle` (`self.WaveStartCountdown`))
  (set `self.NextWaveCountdownTime` (`self.DefaultNextWaveCountdownTime`))
  (set `self.NumberReadyPlayers` 0))

(event `RegisterLogout`
  (params (`Exiting PlayerState` :type "PlayerState Object Reference"))
  ;[1 1 1] Party List Information
  ;;[1 1 1] When a player leaves, remove their icon
  (bind _asplayer_state_1main (cast `/Game/Blueprints/AllLevels/PlayerState1Main` `Exiting PlayerState`))
  (`KismetArrayLibrary.Array_RemoveItem` (`self.ConnectedPlayersGS`) _asplayer_state_1main))

(event `AllPlayersReadyStartWave`
  ;[1 1 1] Start/Stop Wave Timer, Update Current Wave
  (set `self.IsAnyPlayerReady?` false)
  (`KismetSystemLibrary.K2_ClearAndInvalidateTimerHandle` (`self.WaveStartCountdown`))
  (bind _aswave_gmupdated (cast `/Game/Blueprints/Gameplay/WaveGMUpdated` (`GameplayStatics.GetGameMode`)))
  (`/Game/Blueprints/Gameplay/WaveGMUpdated.StartNextWave` _aswave_gmupdated)
  (set `self.NextWaveCountdownTime` (`self.DefaultNextWaveCountdownTime`))
  (set `self.NumberReadyPlayers` 0))

(event `AddLobbyReadyWBClients`
  (params (InName :type Name) (SelectedDifficulty :type "/Game/Blueprints/AllLevels/Variables/Enums/Difficulties Enum" :default "NewEnumerator0"))
  (bind _outactors (`GameplayStatics.GetAllActorsOfClass` "/Game/Blueprints/AllLevels/PlayerControllerMain.PlayerControllerMain_C"))
  (for _array_element _outactors
    (`/Game/Blueprints/AllLevels/PlayerControllerMain.AddLobbyReadyWB` _array_element))
  (set `self.SelectedMap` (`KismetTextLibrary.Conv_NameToText` InName))
  (set `self.SelectedDifficulty` SelectedDifficulty))

(event `StartWaveMode`
  ;[1 1 1] Called when everyone's ready, transitions from lobby to wave mode
  (bind _asfpgmupdated (cast `/Game/Blueprints/Gameplay/FPGMUpdated` (`GameplayStatics.GetGameMode`)))
  (`/Game/Blueprints/Gameplay/FPGMUpdated.TellClientsToTravelMap` _asfpgmupdated)
  (bind _asadvanced_sessions_game_instance_main (cast `/Game/Blueprints/AllLevels/AdvancedSessionsGameInstanceMain` (`GameplayStatics.GetGameInstance`)))
  (set `/Game/Blueprints/AllLevels/AdvancedSessionsGameInstanceMain.Difficulty` (`self.SelectedDifficulty`) _asadvanced_sessions_game_instance_main)
  (set `/Game/Blueprints/AllLevels/AdvancedSessionsGameInstanceMain.NumberOfPlayersJoining` (`AdvancedSessionsLibrary.GetNumberOfNetworkPlayers`) _asadvanced_sessions_game_instance_main)
  (`KismetSystemLibrary.Delay` 2.0)
  (set `self.NumberReadyPlayers` 0)
  (bind _outactors (`GameplayStatics.GetAllActorsOfClass` "/Game/Blueprints/AllLevels/PlayerState1Main.PlayerState1Main_C"))
  (for _array_element _outactors
    (set `/Game/Blueprints/AllLevels/PlayerState1Main.PlayerIsReady?` false _array_element))
  (bind _outactors_2 (`GameplayStatics.GetAllActorsOfClass` "/Game/Blueprints/AllLevels/PlayerControllerMain.PlayerControllerMain_C"))
  (for _array_element_2 _outactors_2
    (`/Game/Blueprints/AllLevels/PlayerControllerMain.SetUnreadyForWaveStartAndLobbyEnd` _array_element_2))
  (`KismetSystemLibrary.Delay` 0.1) ; Don't really know if this needs to be here, but I'm putting it in to make sure all the code gets run before we travel
  (`KismetSystemLibrary.ExecuteConsoleCommand` (`KismetStringLibrary.Concat_StrStr` "ServerTravel " (`KismetTextLibrary.Conv_TextToString` (`self.SelectedMap`))) (`GameplayStatics.GetPlayerController` 0)))

(fn `UserConstructionScript`)