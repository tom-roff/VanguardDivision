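; Thrown Infiltrator grenade that detonates on impact or after a short fuse into a timed cloud disrupting enemies.
; Detonation hides the mesh, starts particle trails, enables the effect area and turns its nav modifier into an obstacle until the actor destroys itself.
; Overlaps stop enemies and toggle their blackboard cloud flag.
; Players gain and lose clamped damage resistance via owner perk checks, which test different perks on enter and exit.
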(event `ExplodeGrenade`
  (`GameplayStatics.SpawnSoundAtLocation` "/Game/Audio/UISounds/Beep2High.Beep2High" (`SceneComponent.K2_GetComponentLocation` (`self.GrenadeMDL`)) (struct) 1.0 1.0 0.0 "/Game/Audio/Attenuations/BaseAtten.BaseAtten" null :!label _label)
  (`SceneComponent.K2_SetWorldRotation` :`self` (`self.GrenadeEffectArea`))
  (`ParticleSystemComponent.BeginTrails` (`self.ParticleSystem`) "None" "None" "ETrailWidthMode_FromCentre" 0.0)
  (`SceneComponent.SetVisibility` (`self.GrenadeMDL`) false false)
  (`PrimitiveComponent.SetCollisionEnabled` (`self.GrenadeEffectArea`) "QueryAndPhysics")
  (`NavModifierComponent.SetAreaClass` (`self.NavModifier`) "/Script/NavigationSystem.NavArea_Obstacle")
  (`KismetSystemLibrary.Delay` (`self.DisruptGrenadeDuration`))
  (`ParticleSystemComponent.EndTrails` (`self.ParticleSystem`))
  (`self.K2_DestroyActor`))

(event `self.ReceiveBeginPlay`
  (`NavModifierComponent.SetAreaClass` (`self.NavModifier`) "/Script/NavigationSystem.NavArea_Default")
  (`PrimitiveComponent.SetCollisionEnabled` (`self.GrenadeEffectArea`) "NoCollision")
  (`KismetSystemLibrary.Delay` 2.5)
  (`PrimitiveComponent.SetSimulatePhysics` (`self.GrenadeMDL`) false)
  (if (not (`self.Has Grenade Exploded?`))
    (set `self.Has Grenade Exploded?` true)
    (goto _label)))

(event `HitServer`
  (set `self.HitComponent` (`.HitComponent` (`GameplayStatics.BreakHitResult` (stale `self.ReceiveHit` Hit))))
  (`PrimitiveComponent.SetSimulatePhysics` (`self.GrenadeMDL`) false)
  (if (not (`self.Has Grenade Exploded?`))
    (set `self.Has Grenade Exploded?` true)
    (`self.ExplodeGrenade`)))

(event `self.ReceiveHit`
  (params (MyComp :type "PrimitiveComponent Object Reference") (Other :type "Actor Object Reference") (OtherComp :type "PrimitiveComponent Object Reference") (bSelfMoved :type Boolean) (HitLocation :type "Vector Structure") (HitNormal :type "Vector Structure") (NormalImpulse :type "Vector Structure") (Hit :type "HitResult Structure (by ref)"))
  (`self.HitServer`))

(event `self.GrenadeEffectArea.OnComponentBeginOverlap`
  (params (OverlappedComponent :type "PrimitiveComponent Object Reference") (OtherActor :type "Actor Object Reference") (OtherComp :type "PrimitiveComponent Object Reference") (OtherBodyIndex :type Integer) (bFromSweep :type Boolean) (SweepResult :type "HitResult Structure (by ref)"))
  (if (== (`GameplayStatics.GetObjectClass` OtherActor) "/Game/TrueFPP/TrueFirstPersonCharacter.TrueFirstPersonCharacter_C")
    (bind _astrue_first_person_character (cast `/Game/TrueFPP/TrueFirstPersonCharacter` (`self.GetOwner`)))
    (if (not (== (`KismetArrayLibrary.Array_Find` (`/Game/TrueFPP/TrueFirstPersonCharacter.PurchasedPerks` _astrue_first_person_character) "NewEnumerator34") -1))
      (bind _astrue_first_person_character_2 (cast `/Game/TrueFPP/TrueFirstPersonCharacter` OtherActor))
      (set `/Game/TrueFPP/TrueFirstPersonCharacter.DamageResistPercentage` (`KismetMathLibrary.FClamp` (+ (`/Game/TrueFPP/TrueFirstPersonCharacter.DamageResistPercentage` _astrue_first_person_character_2) 0.25) 0.0 0.75) _astrue_first_person_character_2))
    (else
      (bind _asenemy_parent (cast `/Game/Blueprints/AIActorsPawns/EnemyParent` OtherActor))
      (bind _returnvalue (`AIBlueprintHelperLibrary.GetBlackboard` _asenemy_parent))
      (`/Engine/EditorBlueprintResources/StandardMacros.IsValid` _returnvalue
        (:`Is Valid`
          (`BlackboardComponent.SetValueAsBool` _returnvalue "IsInInfilCloud?" true))
        (:`Is Not Valid`
          _))
      (`MovementComponent.StopMovementImmediately` (`Character.CharacterMovement` _asenemy_parent)))))

(event `self.GrenadeEffectArea.OnComponentEndOverlap`
  (params (OverlappedComponent :type "PrimitiveComponent Object Reference") (OtherActor :type "Actor Object Reference") (OtherComp :type "PrimitiveComponent Object Reference") (OtherBodyIndex :type Integer))
  (if (== (`GameplayStatics.GetObjectClass` OtherActor) "/Game/TrueFPP/TrueFirstPersonCharacter.TrueFirstPersonCharacter_C")
    (bind _astrue_first_person_character (cast `/Game/TrueFPP/TrueFirstPersonCharacter` (`self.GetOwner`)))
    (if (not (== (`KismetArrayLibrary.Array_Find` (`/Game/TrueFPP/TrueFirstPersonCharacter.PurchasedPerks` _astrue_first_person_character) "NewEnumerator15") -1))
      (bind _astrue_first_person_character_2 (cast `/Game/TrueFPP/TrueFirstPersonCharacter` OtherActor))
      (set `/Game/TrueFPP/TrueFirstPersonCharacter.DamageResistPercentage` (`KismetMathLibrary.FClamp` (+ (`/Game/TrueFPP/TrueFirstPersonCharacter.DamageResistPercentage` _astrue_first_person_character_2) -0.25) 0.0 0.75) _astrue_first_person_character_2))
    (else
      (bind _asenemy_parent (cast `/Game/Blueprints/AIActorsPawns/EnemyParent` OtherActor))
      (if (not (`/Game/Blueprints/AIActorsPawns/EnemyParent.IsDead?` _asenemy_parent))
        (bind _returnvalue (`AIBlueprintHelperLibrary.GetBlackboard` _asenemy_parent))
        (`/Engine/EditorBlueprintResources/StandardMacros.IsValid` _returnvalue
          (:`Is Valid`
            (`BlackboardComponent.SetValueAsBool` _returnvalue "IsInInfilCloud?" false)))))))

(fn `UserConstructionScript`)