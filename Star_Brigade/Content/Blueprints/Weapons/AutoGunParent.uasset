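; Parent Blueprint for automatic guns that fire repeatedly between the player's fire and stop-fire events.
; A fire press shoots once, then starts a looping timer at the weapon's fire rate that plays effects and calls the parent fire logic.
; Releasing fire clears the timer, while an empty magazine clears it and triggers a reload.
; A ResetTimer event restarts the firing timer.
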(event `self.ResetTimer`
  (`KismetSystemLibrary.K2_ClearAndInvalidateTimerHandle` (`self.AutoGunFireTimer`))
  ;[1 1 1] Automatic Firing Logic
  (bind _returnvalue (`KismetSystemLibrary.K2_SetTimerDelegate` (delegate `GunAutoFire`) (`.FireRate_4_51F4EBCF4AE1EC03E8901F8D84AF13C8` (break `/Game/Blueprints/Weapons/WeaponStats` (`self.WeaponStats`))) true :!label _label))
  (set `self.AutoGunFireTimer` _returnvalue))

(event `self.PlayerFireRecieve`
  ;[1 1 1] Automatic Firing Logic
  (if (> (`self.CurrentAmmoInMag`) 0)
    (`self.GunAutoFire`)
    (goto _label)
    (else
      (`self.ReloadAutoGun`))))

(event `GunAutoFire`
  ;[1 1 1] Automatic Firing Logic
  (if (> (`self.CurrentAmmoInMag`) 0)
    (`self.DoGunFX`)
    (`self.Fire Gun Parent`)
    (if (not (> (`self.CurrentAmmoInMag`) 0))
      (`self.ReloadAutoGun`))
    (else
      (`self.ReloadAutoGun`))))

(event `Player Stop Fire Receive`
  (bind _autogunfiretimer (`self.AutoGunFireTimer`))
  ;[1 1 1] Automatic Firing Logic
  (if (`KismetSystemLibrary.K2_IsValidTimerHandle` _autogunfiretimer)
    (`KismetSystemLibrary.K2_ClearAndInvalidateTimerHandle` _autogunfiretimer)))

(event `ReloadAutoGun`
  (bind _autogunfiretimer (`self.AutoGunFireTimer`))
  ;[1 1 1] Automatic Firing Logic
  (if (`KismetSystemLibrary.K2_IsValidTimerHandle` _autogunfiretimer)
    (`KismetSystemLibrary.K2_ClearAndInvalidateTimerHandle` _autogunfiretimer))
  (`self.Reload Gun`))

(fn `UserConstructionScript`)