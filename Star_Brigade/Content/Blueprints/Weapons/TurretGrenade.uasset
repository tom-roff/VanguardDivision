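; TurretGrenade is a grenade projectile, by its name fired by a turret, that explodes on impact.
; On hit, unless it strikes a LauncherGrenade1 or TrueFirstPersonCharacter, it applies radial explosive damage with falloff, spawns a scaled particle effect and destroys itself.
; The blast ignores every TrueFirstPersonCharacter in the level and credits the damage to the owning pawn's controller.
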(event `self.ReceiveHit`
  (params (MyComp :type "PrimitiveComponent Object Reference") (Other :type "Actor Object Reference") (OtherComp :type "PrimitiveComponent Object Reference") (bSelfMoved :type Boolean) (HitLocation :type "Vector Structure") (HitNormal :type "Vector Structure") (NormalImpulse :type "Vector Structure") (Hit :type "HitResult Structure (by ref)"))
  (bind _returnvalue (`GameplayStatics.GetObjectClass` (`.HitActor` (`GameplayStatics.BreakHitResult` Hit))))
  (if (and (!= _returnvalue "/Game/Blueprints/Weapons/LauncherGrenade1.LauncherGrenade1_C") (!= _returnvalue "/Game/TrueFPP/TrueFirstPersonCharacter.TrueFirstPersonCharacter_C"))
    (bind _outactors (`GameplayStatics.GetAllActorsOfClass` "/Game/TrueFPP/TrueFirstPersonCharacter.TrueFirstPersonCharacter_C"))
    (`GameplayStatics.ApplyRadialDamageWithFalloff` (`self.Damage`) 20.0 HitLocation 200.0 300.0 0.5 "/Game/Blueprints/Gameplay/ExplosiveDamageType.ExplosiveDamageType_C" _outactors self (`Pawn.GetController` (cast `Pawn` (`self.GetOwner`) :!pure true)))
    (`GameplayStatics.SpawnEmitterAtLocation` "/Game/Particles/VFX_Toolkit_V1/GrenadeFX.GrenadeFX" HitLocation (struct) (2.3 2.3 2.3))
    (`self.K2_DestroyActor`)))

(fn `UserConstructionScript`)