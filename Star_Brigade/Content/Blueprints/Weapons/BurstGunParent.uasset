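; Parent Blueprint for burst-fire guns, firing a short burst of two or three shots per trigger press.
; PlayerFire, gated by reload and recent-fire flags, chains FireGun calls spaced by the fire rate, with BulletsInBurst enabling the third shot.
; An empty magazine triggers a reload; otherwise FireDelay must pass before the next burst.
; FireGun sets the recent-fire flag and defers to its parent implementation, while the Construction Script sets default weapon stats.
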(event `/Game/Blueprints/Interfaces/PlayerInterface.PlayerFire`
  (params (`Controller Firing` :type "PlayerController Object Reference"))
  (bind (_damage _firerate) (break `/Game/Blueprints/Weapons/WeaponStats` (`self.WeaponStats`)))
  (if (`self.IsReloading?`)
    _
    (elif (`self.RecentlyFired?`)
      _
      (elif (> (`self.CurrentAmmoInMag`) 0)
        (`self.FireGun`)
        (if (> (`self.CurrentAmmoInMag`) 0)
          (`KismetSystemLibrary.Delay` _firerate)
          (`self.FireGun`)
          (if (> (`self.CurrentAmmoInMag`) 0)
            (if (>= (`self.BulletsInBurst`) 3)
              (`KismetSystemLibrary.Delay` _firerate)
              (`self.FireGun`))
            (if (> (`self.CurrentAmmoInMag`) 0)
              (`KismetSystemLibrary.Delay` (`self.FireDelay`))
              (set `self.RecentlyFired?` false)
              (else
                (`self.Reload Gun`)
                (set `self.RecentlyFired?` false)))
            (else
              (`self.Reload Gun`)
              (set `self.RecentlyFired?` false)))
          (else
            (`self.Reload Gun`)
            (set `self.RecentlyFired?` false)))
        (else
          (`self.Reload Gun`)
          (set `self.RecentlyFired?` false))))))

(event `FireGun`
  (set `self.RecentlyFired?` true)
  (`self.Fire Gun Parent`))

(fn `UserConstructionScript`
  (set `self.WeaponStats` (make `/Game/Blueprints/Weapons/WeaponStats` 4.0 0.09 4.0)))