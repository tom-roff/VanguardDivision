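; Base gun Blueprint for the first-person character, handling hitscan fire, ammo, reloading, spread, recoil and effects, with hooks for AutoGunParent.
; Firing runs through a DoOnce fire-rate gate into a cone-randomized camera trace, which feeds impact FX, damage, hitmarkers and recoil.
; Spread grows per shot and decays on a looping timer by movement and ADS state.
; Perks, Gauss state and a temporary Overloader boost modify damage, ammo, reload and fire rate.
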(event `ResetTimer`)

(event `OverloaderFireRate`
  (bind (_damage _firerate _reloadspeed _maxammototal _maxammopermag _verticalrecoil _horizontalrecoil _adsfov _adsspeedmultiplier _weaponspreadidle _weaponspreadrunning _weaponspreadfiringmax) (break `/Game/Blueprints/Weapons/WeaponStats` (`self.WeaponStats`)))
  (bind (_damage_2 _firerate_2 _reloadspeed_2 _maxammototal_2 _maxammopermag_2 _verticalrecoil_2 _horizontalrecoil_2 _adsfov_2 _adsspeedmultiplier_2 _weaponspreadidle_2 _weaponspreadrunning_2 _weaponspreadfiringmax_2) (break `/Game/Blueprints/Weapons/WeaponStats` (`self.WeaponStats`)))
  (set `self.WeaponStats` (make `/Game/Blueprints/Weapons/WeaponStats` _damage (/ (* _firerate 2.0) 3.0) _reloadspeed _maxammototal _maxammopermag _verticalrecoil _horizontalrecoil _adsfov _adsspeedmultiplier _weaponspreadidle _weaponspreadrunning _weaponspreadfiringmax))
  (`self.ResetTimer`)
  (`KismetSystemLibrary.Delay` 5.0)
  (set `self.WeaponStats` (make `/Game/Blueprints/Weapons/WeaponStats` _damage_2 (* _firerate_2 1.5) _reloadspeed_2 _maxammototal_2 _maxammopermag_2 _verticalrecoil_2 _horizontalrecoil_2 _adsfov_2 _adsspeedmultiplier_2 _weaponspreadidle_2 _weaponspreadrunning_2 _weaponspreadfiringmax_2))
  (`self.ResetTimer`))

(event `DoGunFX`
  (bind _returnvalue (`self.GetOwner`))
  ;[1 1 1] Gun FX Client
  (`ParticleSystemComponent.BeginTrails` (`self.ParticleSystem`) "None" "None" "ETrailWidthMode_FromCentre" 0.0)
  (`GameplayStatics.PlaySoundAtLocation` (`self.WeaponFireSound`) (`self.K2_GetActorLocation` _returnvalue) (struct) 1.0 (select `bool` (`/Game/TrueFPP/TrueFirstPersonCharacter.IsGaussed?` (cast `/Game/TrueFPP/TrueFirstPersonCharacter` _returnvalue :!pure true)) :`false` 1.0 :`true` 0.7 :!type "Float (single-precision)") 0.0 "/Game/Audio/Attenuations/BaseAtten.BaseAtten" null _returnvalue)
  (`PlayerCameraManager.StartMatineeCameraShake` :`self` (`GameplayStatics.GetPlayerCameraManager` 0) :`ShakeClass` "/Game/Blueprints/CameraShakes/WeaponFireShakeSmall.WeaponFireShakeSmall_C")
  (`|PlayMontage` (`/Game/TrueFPP/TrueFirstPersonCharacter.FPCharMesh` (cast `/Game/TrueFPP/TrueFirstPersonCharacter` (`self.GetOwner`) :!pure true)) "/Game/FirstPerson/Animations/FirstPersonFire_Montage.FirstPersonFire_Montage"))

(event `/Game/Blueprints/Interfaces/WeaponInterface.Reload`
  (if (`self.IsReloading?`)
    _
    (elif (< (`self.CurrentAmmoInMag`) (`.MaxAmmoPerMag_11_EE96499142276B13A758FFAF0727435C` (break `/Game/Blueprints/Weapons/WeaponStats` (`self.WeaponStats`))))
      (`self.Reload Gun`))))

(event `/Game/Blueprints/Interfaces/AmmoInterface.AmmoUpdate`
  (bind (_damage _firerate _reloadspeed _maxammototal _maxammopermag) (break `/Game/Blueprints/Weapons/WeaponStats` (`self.WeaponStats`)))
  ;[1 1 1] When Called, Refill Ammo
  (set `self.CurrentAmmoTotal` _maxammototal)
  (set `self.CurrentAmmoInMag` _maxammopermag :!pinned true) ; This could be disabled later for balancing reasons
)

(event `Reload Gun`
  (bind (_damage _firerate _reloadspeed _maxammototal _maxammopermag) (break `/Game/Blueprints/Weapons/WeaponStats` (`self.WeaponStats`)))
  ;[1 1 1] Reloading System
  (if (`self.IsReloading?`)
    _
    (elif (> (`self.CurrentAmmoTotal`) 0)
      (bind _asauto_gun_parent (cast `/Game/Blueprints/Weapons/AutoGunParent` self)
        (:`then`
          (`KismetSystemLibrary.K2_ClearAndInvalidateTimerHandle` (`/Game/Blueprints/Weapons/AutoGunParent.AutoGunFireTimer` _asauto_gun_parent)))
        (:`CastFailed`
          _))
      (`KismetSystemLibrary.PrintString` "Reloading...")
      (set `self.IsReloading?` true)
      (bind _astrue_first_person_character (cast `/Game/TrueFPP/TrueFirstPersonCharacter` (`self.GetOwner`)))
      (if (`/Game/TrueFPP/TrueFirstPersonCharacter.IsADSing?` _astrue_first_person_character)
        (`/Game/TrueFPP/TrueFirstPersonCharacter.GetOutOfADS` _astrue_first_person_character))
      (if (`KismetArrayLibrary.Array_Contains` (`/Game/TrueFPP/TrueFirstPersonCharacter.PurchasedPerks` _astrue_first_person_character) "NewEnumerator1")
        (`KismetSystemLibrary.Delay` (* _reloadspeed 0.7))
        (else
          (`KismetSystemLibrary.Delay` _reloadspeed)))
      (set `self.CurrentAmmoTotalPreSet` (`self.CurrentAmmoTotal`))
      (set `self.CurrentMagTotalPreSet` (`self.CurrentAmmoInMag`))
      (set `self.CurrentAmmoTotal` (`KismetMathLibrary.Clamp` (- (`self.CurrentAmmoTotal`) (- _maxammopermag (`self.CurrentAmmoInMag`))) 0 _maxammototal))
      (set `self.CurrentAmmoInMag` (`KismetMathLibrary.Clamp` _maxammopermag 0 (+ (`self.CurrentMagTotalPreSet`) (`self.CurrentAmmoTotalPreSet`))))
      (set `self.IsReloading?` false)
      (`KismetSystemLibrary.PrintString` "Gun Reloaded")
      (`self.ResetFireReload`))))

(event `PlayerFireRecieve`
  ;[1 1 1] When this gun receives the message from the player to fire, do the line trace and send to the game state to fire
  (`self.DoGunFX`)
  (`self.Fire Gun Parent`)
  (if (not (> (`self.CurrentAmmoInMag`) 0))
    (`self.Reload Gun`)))

(event `Fire Gun Parent`
  (bind (_weaponstats_damage _weaponstats_firerate _weaponstats_reloadspeed _weaponstats_maxammototal _weaponstats_maxammopermag _weaponstats_verticalrecoil _weaponstats_horizontalrecoil _weaponstats_adsfov _weaponstats_adsspeedmultiplier _weaponstats_weaponspreadidle _weaponstats_weaponspreadrunning _weaponstats_weaponspreadfiringmax) (break `/Game/Blueprints/Weapons/WeaponStats` (`self.WeaponStats`)))
  ;[1 1 1] When this gun receives the message from the player to fire, do the line trace and send to the game state to fire
  (`/Engine/EditorBlueprintResources/StandardMacros.DoOnce` false :!label _label
    (:`Completed`
      (set `self.CurrentSpreadAngle` (`KismetMathLibrary.FClamp` (+ (`self.CurrentSpreadAngle`) 0.07) 0.0 _weaponstats_weaponspreadfiringmax))
      (`self.DoLineTrace`)
      (bind (_bblockinghit _binitialoverlap _time _distance _location _impactpoint _normal _impactnormal _physmat _hitactor _hitcomponent _hitbonename) (`GameplayStatics.BreakHitResult` (stale `DoLineTrace` _outhit)))
      (`self.PlayWeaponFXMulti` _location _impactnormal)
      (`self.ServerShoot`)
      (`KismetSystemLibrary.Delay` (- (`.FireRate_4_51F4EBCF4AE1EC03E8901F8D84AF13C8` (break `/Game/Blueprints/Weapons/WeaponStats` (`self.WeaponStats`))) 0.02))
      (goto _label :!via `Reset`))))

(event `ResetFireReload`
  ;[1 1 1] When this gun receives the message from the player to fire, do the line trace and send to the game state to fire
  (goto _label :!via `Reset`))

(event `TellClientDoHitmarker`
  (params (`Hit Head?` :type Boolean))
  (bind _crosshairui (`/Game/UI_elements/GameplayWBs/FPCharHUD.CrosshairUI` (`/Game/TrueFPP/TrueFirstPersonCharacter.HealthBarRef` (cast `/Game/TrueFPP/TrueFirstPersonCharacter` (`self.GetOwner`) :!pure true))))
  ;[1 1 1] Server Side Shooting
  (if `Hit Head?`
    (`/Game/UI_elements/GameplayWBs/CrosshairUI.HitMarkerHeadShot` _crosshairui)
    (else
      (`/Game/UI_elements/GameplayWBs/CrosshairUI.HitMarkerBodyShot` _crosshairui))))

(event `ServerShoot`
  (bind _damage (break `/Game/Blueprints/Weapons/WeaponStats` (`self.WeaponStats`)))
  (bind _astrue_first_person_character (cast `/Game/TrueFPP/TrueFirstPersonCharacter` (`self.GetOwner`) :!pure true))
  (bind _returnvalue (select `bool` (`self.HitCritPt?`) :`false` _damage :`true` (* _damage (select `bool` (`KismetArrayLibrary.Array_Contains` (`/Game/TrueFPP/TrueFirstPersonCharacter.PurchasedPerks` _astrue_first_person_character) "NewEnumerator4") :`false` 1.5 :`true` 3.0 :!type "Float (single-precision)"))))
  ;[1 1 1] Server Side Shooting
  (bind _asenemy_parent (cast `/Game/Blueprints/AIActorsPawns/EnemyParent` (`self.Weapon Hit Actor`))
    (:`then`
      (bind _output_get (set `/Game/Blueprints/AIActorsPawns/EnemyParent.Hit Bone` (`self.Weapon Hit Bone`) _asenemy_parent))
      (if (`/Game/Blueprints/AIActorsPawns/EnemyParent.IsDead?` _asenemy_parent)
        (`/Game/Blueprints/AIActorsPawns/EnemyParent.PlayHitSound` _asenemy_parent false)
        (else
          (bind _returnvalue_2 (== _output_get "head"))
          (`/Game/Blueprints/AIActorsPawns/EnemyParent.PlayHitSound` _asenemy_parent _returnvalue_2)
          (`self.TellClientDoHitmarker` _returnvalue_2))))
    (:`CastFailed`
      _))
  (`GameplayStatics.ApplyDamage` (`self.Weapon Hit Actor`) (select `bool` (`/Game/TrueFPP/TrueFirstPersonCharacter.IsGaussed?` _astrue_first_person_character) :`false` _returnvalue :`true` (* _returnvalue 2.0)) (`Pawn.GetController` _astrue_first_person_character) self "/Game/Blueprints/Gameplay/SmallArmsDamageType.SmallArmsDamageType_C")
  (set `self.CurrentAmmoInMag` (- (`self.CurrentAmmoInMag`) 1))
  (`self.SetRecoilClient`))

(event `DecreaseSpread`
  (bind (_weaponstats_damage _weaponstats_firerate _weaponstats_reloadspeed _weaponstats_maxammototal _weaponstats_maxammopermag _weaponstats_verticalrecoil _weaponstats_horizontalrecoil _weaponstats_adsfov _weaponstats_adsspeedmultiplier _weaponstats_weaponspreadidle _weaponstats_weaponspreadrunning) (break `/Game/Blueprints/Weapons/WeaponStats` (`self.WeaponStats`)))
  (bind _returnvalue (* (`self.CurrentSpreadAngle`) 0.9))
  ;[1 1 1] When this gun receives the message from the player to fire, do the line trace and send to the game state to fire
  (bind _astrue_first_person_character (cast `/Game/TrueFPP/TrueFirstPersonCharacter` (`self.GetOwner`)))
  (if (`/Game/TrueFPP/TrueFirstPersonCharacter.IsADSing?` _astrue_first_person_character)
    (set `self.CurrentSpreadAngle` 0.0)
    (else
      (bind _asauto_gun_parent (cast `/Game/Blueprints/Weapons/AutoGunParent` self)
        (:`then`
          (if (not (`KismetSystemLibrary.K2_IsValidTimerHandle` (`/Game/Blueprints/Weapons/AutoGunParent.AutoGunFireTimer` _asauto_gun_parent)))
            (if (>= (`KismetMathLibrary.VSize` (`self.GetVelocity` (`self.GetOwner`))) 100.0) :!label _label_2
              (set `self.CurrentSpreadAngle` (`KismetMathLibrary.FClamp` _returnvalue _weaponstats_weaponspreadrunning 1000.0))
              (else
                (set `self.CurrentSpreadAngle` (`KismetMathLibrary.FClamp` _returnvalue _weaponstats_weaponspreadidle 1000.0))))))
        (:`CastFailed`
          (goto _label_2))))))

(event `self.ReceiveBeginPlay`
  ;[1 1 1] Ammo counter text updating and spread decrease timer start
  (`self.StartSpreadDecreaseTimer`)
  (bind _astrue_first_person_character (cast `/Game/TrueFPP/TrueFirstPersonCharacter` (`self.GetOwner`)))
  (add `/Game/TrueFPP/TrueFirstPersonCharacter.PlayerFired` _astrue_first_person_character (delegate `PlayerShotFromGun1`))
  (`self.SetExtraMagsPerk`))

(event `SetExtraMagsPerk`
  (bind (_damage _firerate _reloadspeed _maxammototal _maxammopermag _verticalrecoil _horizontalrecoil) (break `/Game/Blueprints/Weapons/WeaponStats` (`self.WeaponStats`)))
  ;[1 1 1] Double Max Ammo if the extra mags perk is purchased
  (bind _astrue_first_person_character (cast `/Game/TrueFPP/TrueFirstPersonCharacter` (`self.GetOwner`)))
  (if (!= (`KismetArrayLibrary.Array_Find` (`/Game/TrueFPP/TrueFirstPersonCharacter.PurchasedPerks` _astrue_first_person_character) "NewEnumerator0") -1)
    (set `self.WeaponStats` (make `/Game/Blueprints/Weapons/WeaponStats` _damage _firerate _reloadspeed (* _maxammototal 2) _maxammopermag _verticalrecoil _horizontalrecoil))))

(event `StartSpreadDecreaseTimer`
  ;[1 1 1] Ammo counter text updating and spread decrease timer start
  (`KismetSystemLibrary.K2_SetTimerDelegate` (delegate `DecreaseSpread`) 0.05 true))

(event `PlayerShotFromGun1`
  ;[1 1 1] Ammo counter text updating and spread decrease timer start
  (if (not (<= (`self.CurrentAmmoTotal`) 0))
    (`self.UpdateText1`)))

(event `SetRecoilClient`
  (bind (_damage _firerate _reloadspeed _maxammototal _maxammopermag _verticalrecoil _horizontalrecoil) (break `/Game/Blueprints/Weapons/WeaponStats` (`self.WeaponStats`)))
  (bind _aspawn (cast `Pawn` (`self.GetOwner`) :!pure true))
  ;[1 1 1] Server Side Shooting
  (`Pawn.AddControllerPitchInput` _aspawn (`KismetMathLibrary.RandomFloatInRange` (* -3.0 _verticalrecoil) _verticalrecoil))
  (`Pawn.AddControllerYawInput` _aspawn (`KismetMathLibrary.RandomFloatInRange` 0.0 (* 3.0 _horizontalrecoil))))

(event `UpdateText1`
  ;[1 1 1] Ammo counter text updating and spread decrease timer start
)

(event `DoLineTrace`
  (bind (_astrue_first_person_character _bsuccess) (cast `/Game/TrueFPP/TrueFirstPersonCharacter` (`self.GetOwner`) :!pure true))
  (bind _returnvalue (`SceneComponent.K2_GetComponentLocation` (`/Game/TrueFPP/TrueFirstPersonCharacter.PlayerCam` _astrue_first_person_character)))
  ;[1 1 1] Line Trace
  (if _bsuccess
    (bind _outhit (`KismetSystemLibrary.LineTraceSingle` _returnvalue (+ (* (`KismetMathLibrary.RandomUnitVectorInConeInDegrees` (`KismetMathLibrary.GetForwardVector` (`Pawn.GetControlRotation` _astrue_first_person_character)) (`self.CurrentSpreadAngle`)) 10000.0) _returnvalue) "TraceTypeQuery4" true))
    (bind (_bblockinghit _binitialoverlap _time _distance _location _impactpoint _normal _impactnormal _physmat _hitactor _hitcomponent _hitbonename) (`GameplayStatics.BreakHitResult` _outhit))
    (set `self.Weapon Hit Actor` _hitactor)
    (set `self.Weapon Hit Bone` _hitbonename)
    (`/Engine/EditorBlueprintResources/StandardMacros.IsValid` _hitcomponent
      (:`Is Valid`
        (if (== _hitbonename "head")
          (set `self.HitCritPt?` true) ; Doesn't need to be replicated because elsewhere it's called from the server too
          (else
            (set `self.HitCritPt?` false)))))))

(event `PlayWeaponFXMulti`
  (params (Location :type "Vector Structure") (`Impact Normal` :type "Vector Structure"))
  (bind _returnvalue (`self.GetOwner`))
  (bind _returnvalue_2 (`GameplayStatics.GetObjectClass` (`self.Weapon Hit Actor`)))
  (bind _astrue_first_person_character (cast `/Game/TrueFPP/TrueFirstPersonCharacter` (`self.GetOwner`) :!pure true))
  ;[1 1 1] Weapon Art FX Multicast
  (`/Game/Blueprints/ParticleFuncs.TracerFireFX` (`SceneComponent.K2_GetComponentLocation` (`self.FireLoc`)) Location)
  (if (not (== (`GameplayStatics.GetPlayerController` 0) (`Pawn.GetController` _astrue_first_person_character)))
    (`GameplayStatics.PlaySoundAtLocation` (`self.WeaponFireSound`) (`self.K2_GetActorLocation` _returnvalue) (struct) 1.0 (select `bool` (`/Game/TrueFPP/TrueFirstPersonCharacter.IsGaussed?` _astrue_first_person_character) :`false` 1.0 :`true` 0.7 :!type "Float (single-precision)") 0.0 "/Game/Audio/Attenuations/BaseAtten.BaseAtten" null _returnvalue))
  (if (`KismetMathLibrary.ClassIsChildOf` _returnvalue_2 "/Script/Engine.Pawn")
    (if (`KismetMathLibrary.ClassIsChildOf` _returnvalue_2 "/Game/Blueprints/AIActorsPawns/EnemyParent.EnemyParent_C")
      (`NiagaraFunctionLibrary.SpawnSystemAtLocation` "/Game/Particles/Sparks_Standard.Sparks_Standard" Location (`KismetMathLibrary.Conv_VectorToRotator` `Impact Normal`)))
    (else
      (`/Game/Blueprints/ParticleFuncs.Bullet Impact FX` Location `Impact Normal`))))

(fn `IfPhysicsApplyForce`
  (bind _asstatic_mesh_actor (cast `StaticMeshActor` (`self.Weapon Hit Actor`)))
  (bind _staticmeshcomponent (`StaticMeshActor.StaticMeshComponent` _asstatic_mesh_actor))
  (if (`SceneComponent.IsSimulatingPhysics` _staticmeshcomponent "None")
    (`PrimitiveComponent.AddImpulse` _staticmeshcomponent (* (`KismetMathLibrary.GetForwardVector` (`KismetMathLibrary.FindLookAtRotation` (`SceneComponent.K2_GetComponentLocation` (`self.FireLoc`)) (`SceneComponent.K2_GetComponentLocation` _staticmeshcomponent))) 4000.0) "None" false)))

(fn `UserConstructionScript`)