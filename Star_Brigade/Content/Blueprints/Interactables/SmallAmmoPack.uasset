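; A placeable ammo pack that periodically resupplies nearby players and can be removed by its owner.
; A looping timer, started from the construction script, finds TrueFirstPersonCharacters overlapping the sphere and tops up their held weapon's total ammo, clamped to that weapon's maximum.
; Look-at events show a removal prompt to the owning pawn's controller and destroy the pack when that owner interacts.
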(event `/Game/Blueprints/Interfaces/PlayerInterface.BeginLookAt`
  (params (`Looking at Controller` :type "PlayerController Object Reference"))
  (if (== `Looking at Controller` (`Pawn.GetController` (cast `Pawn` (`self.GetOwner`) :!pure true)))
    (`/Game/Blueprints/AllLevels/PlayerControllerMain.ShowInteractWB` (cast `/Game/Blueprints/AllLevels/PlayerControllerMain` `Looking at Controller` :!pure true) "Remove Ammo Pack")))

(event `/Game/Blueprints/Interfaces/PlayerInterface.EndLookAt`
  (params (LookingAtController :type "PlayerController Object Reference"))
  (`/Game/Blueprints/AllLevels/PlayerControllerMain.RemoveInteractWB` (cast `/Game/Blueprints/AllLevels/PlayerControllerMain` LookingAtController :!pure true)))

(event `SetTimerFirstTime`
  (bind _returnvalue (`KismetSystemLibrary.K2_SetTimerDelegate` (delegate `GiveAmmo`) (`self.AmmoGiveTime`) true))
  (set `self.GiveAmmoTimer` _returnvalue))

(event `GiveAmmo`
  (bind _outactors (`KismetSystemLibrary.ComponentOverlapActors` (`self.Sphere`) (`SceneComponent.K2_GetComponentToWorld` (`self.Sphere`)) (`|MakeArray` "ObjectTypeQuery3" :!type "EObjectTypeQuery Enum") "/Game/TrueFPP/TrueFirstPersonCharacter.TrueFirstPersonCharacter_C"))
  (for _array_element _outactors
    (bind _astrue_first_person_character (cast `/Game/TrueFPP/TrueFirstPersonCharacter` _array_element))
    (bind _asgun_parent (cast `/Game/Blueprints/Weapons/GunParent` (`/Game/TrueFPP/TrueFirstPersonCharacter.CurrentWeaponInHand` _astrue_first_person_character)))
    (set `/Game/Blueprints/Weapons/GunParent.CurrentAmmoTotal` (`KismetMathLibrary.Clamp` (+ (`/Game/Blueprints/Weapons/GunParent.CurrentAmmoTotal` _asgun_parent) 5) 0 (`.MaxAmmoTotal_12_8E6D339A4234F206186293B651EF05A5` (break `/Game/Blueprints/Weapons/WeaponStats` (`/Game/Blueprints/Weapons/GunParent.WeaponStats` _asgun_parent)))) _asgun_parent)))

(event `/Game/Blueprints/Interfaces/PlayerInterface.LookingAt`
  (params (LookingAtController :type "PlayerController Object Reference"))
  ;[1 1 1] Destroying
  (if (== LookingAtController (`Pawn.GetController` (cast `Pawn` (`self.GetOwner`) :!pure true)))
    (`PrimitiveComponent.SetCollisionResponseToAllChannels` (`self.BaseBox`) "ECR_Ignore")
    (`self.SetActorEnableCollision` self false)
    (`self.K2_DestroyActor`)))

(fn `OnRep_IsBeingDestroyed?`
  (if true
    (`self.K2_DestroyActor`)))

(fn `UserConstructionScript`
  (`self.SetTimerFirstTime`))