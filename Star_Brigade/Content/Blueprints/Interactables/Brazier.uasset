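; Interactable brazier that toggles on and off through the Lookingat event and burns the player while lit.
; When lit, it starts the Fire trails and a looping timer that randomizes FireLight intensity, with the interval rolled once per ignition.
; FireHitBox overlap runs a repeating damage timer on TrueFirstPersonCharacter until overlap ends.
; An OnRep for BrazierOff mirrors the visuals, but its timer targets "FlickerLight", a name not defined here.
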(event `LightFlickerFunction`
  ;[1 1 1] Light Flicker Functionality
  (`ParticleSystemComponent.BeginTrails` (`self.Fire`) "None" "None" "ETrailWidthMode_FromFirst" 0.0)
  (`LightComponent.SetIntensity` (`self.FireLight`) 40000.0)
  (bind _returnvalue (`KismetSystemLibrary.K2_SetTimerDelegate` (delegate `Lightflicker`) (`KismetMathLibrary.RandomFloatInRange` 0.01 0.5) true)))

(event `Lightflicker`
  ;[1 1 1] Light Flicker Functionality
  (`LightComponent.SetIntensity` (`self.FireLight`) (`KismetMathLibrary.RandomFloatInRange` 30000.0 60000.0)))

(event `/Game/Blueprints/Interfaces/PlayerInterface.LookingAt`
  (params (LookingAtController :type "PlayerController Object Reference"))
  ;[1 1 1] On/Off Function System
  (if (`self.BrazierOff?`)
    (set `self.BrazierOff?` false)
    (`self.LightFlickerFunction`)
    (else
      (set `self.BrazierOff?` true)
      (`LightComponent.SetIntensity` (`self.FireLight`) 0.0)
      (`ParticleSystemComponent.EndTrails` (`self.Fire`))
      (`KismetSystemLibrary.K2_ClearAndInvalidateTimerHandle` (stale `LightFlickerFunction` _returnvalue)))))

(event `self.FireHitBox.OnComponentBeginOverlap`
  (params (OverlappedComponent :type "PrimitiveComponent Object Reference") (OtherActor :type "Actor Object Reference") (OtherComp :type "PrimitiveComponent Object Reference") (OtherBodyIndex :type Integer) (bFromSweep :type Boolean) (SweepResult :type "HitResult Structure (by ref)"))
  ;[1 1 1] Deal Damage to Player if They're Standing in Fire
  (bind _returnvalue (`KismetSystemLibrary.K2_SetTimerDelegate` (delegate `DealDamage`) 0.5 true)) ; Basically just a loop that stops when we end overlap
)

(event `DealDamage`
  ;[1 1 1] Deal Damage to Player if They're Standing in Fire
  (if (not (`self.BrazierOff?`))
    (bind _astrue_first_person_character (cast `/Game/TrueFPP/TrueFirstPersonCharacter` (stale `self.FireHitBox.OnComponentBeginOverlap` OtherActor)))
    (`GameplayStatics.ApplyDamage` _astrue_first_person_character 5.0 null self)))

(event `self.FireHitBox.OnComponentEndOverlap`
  (params (OverlappedComponent :type "PrimitiveComponent Object Reference") (OtherActor :type "Actor Object Reference") (OtherComp :type "PrimitiveComponent Object Reference") (OtherBodyIndex :type Integer))
  ;[1 1 1] Deal Damage to Player if They're Standing in Fire
  (`KismetSystemLibrary.K2_ClearAndInvalidateTimerHandle` (stale `self.FireHitBox.OnComponentBeginOverlap` _returnvalue)))

(fn `OnRep_BrazierOff?`
  (if (`self.BrazierOff?`)
    (set `self.BrazierOff?` true)
    (`LightComponent.SetIntensity` (`self.FireLight`) 0.0)
    (`ParticleSystemComponent.EndTrails` (`self.Fire`))
    (else
      (set `self.BrazierOff?` false)
      (`ParticleSystemComponent.BeginTrails` (`self.Fire`) "None" "None" "ETrailWidthMode_FromFirst" 0.0)
      (`KismetSystemLibrary.K2_SetTimer` null "FlickerLight" (`KismetMathLibrary.RandomFloatInRange` 0.0 0.5) true))))

(fn `UserConstructionScript`)