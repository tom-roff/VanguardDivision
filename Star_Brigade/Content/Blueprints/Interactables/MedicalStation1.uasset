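; MedicalStation1 is a wall-or-world health station interactable that heals the first-person player by 25.
; BeginLookat and EndLookat show and remove a prompt widget reading "Refill Health" or "Health Full".
; Lookingat triggers HealthStationInteract when health is below 100, which heals, updates health values and plays a sound.
; A DoOnce gates reuse while PivotPoint eases to a rotated pose and back around a three-second delay.
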(event `HealthStationInteract`
  (bind _astrue_first_person_character (cast `/Game/TrueFPP/TrueFirstPersonCharacter` (`GameplayStatics.GetPlayerCharacter` 0)))
  (if (not (`self.HealthIsFull?`))
    (`/Engine/EditorBlueprintResources/StandardMacros.DoOnce` false :!label _label
      (:`Completed`
        (`/Game/TrueFPP/TrueFirstPersonCharacter.HealPlayer` _astrue_first_person_character 25)
        (`/Game/TrueFPP/TrueFirstPersonCharacter.UpdateHealthValues` _astrue_first_person_character)
        (`GameplayStatics.PlaySoundAtLocation` "/Game/Audio/switchgood.switchgood" (`self.K2_GetActorLocation`) (struct) 1.0 1.0 0.0 null null null)
        (`KismetSystemLibrary.MoveComponentTo` (`self.pivotPoint`) (26.350719 -7.318058 39.725052) (struct :`Yaw` 120.0) true)
        (`KismetSystemLibrary.Delay` 3.0)
        (`KismetSystemLibrary.MoveComponentTo` (`self.pivotPoint`) (26.350719 -7.318058 39.725052) (struct) false true)
        (goto _label :!via `Reset`)))))

(event `/Game/Blueprints/Interfaces/PlayerInterface.LookingAt`
  (params (LookingAtController :type "PlayerController Object Reference"))
  (bind _astrue_first_person_character (cast `/Game/TrueFPP/TrueFirstPersonCharacter` (`GameplayStatics.GetPlayerCharacter` 0)))
  (if (< (`KismetMathLibrary.Conv_IntToDouble` (`/Game/TrueFPP/TrueFirstPersonCharacter.CurrentHealth` _astrue_first_person_character)) 100.0)
    (`self.HealthStationInteract`)))

(event `/Game/Blueprints/Interfaces/PlayerInterface.BeginLookAt`
  (params (`Looking at Controller` :type "PlayerController Object Reference"))
  (bind _astrue_first_person_character (cast `/Game/TrueFPP/TrueFirstPersonCharacter` (`GameplayStatics.GetPlayerCharacter` 0)))
  (`/Engine/EditorBlueprintResources/StandardMacros.IsValid` (`self.RefillHealthWB1`)
    (:`Is Valid`
      _)
    (:`Is Not Valid`
      (bind _returnvalue (`|CreateWidget` "/Game/UI_elements/GameplayWBs/BaseLookingAtUI.BaseLookingAtUI_C" (`GameplayStatics.GetPlayerController` 0)))
      (bind _output_get (set `self.RefillHealthWB1` _returnvalue))))
  (if (< (`/Game/TrueFPP/TrueFirstPersonCharacter.CurrentHealth` _astrue_first_person_character) 100)
    (set `/Game/UI_elements/GameplayWBs/BaseLookingAtUI.TextToShow` "Refill Health" _output_get)
    (else
      (set `/Game/UI_elements/GameplayWBs/BaseLookingAtUI.TextToShow` "Health Full" (`self.RefillHealthWB1`))))
  (`UserWidget.AddToViewport` _output_get 0))

(event `/Game/Blueprints/Interfaces/PlayerInterface.EndLookAt`
  (params (LookingAtController :type "PlayerController Object Reference"))
  (bind _refillhealthwb1 (`self.RefillHealthWB1`))
  (`/Engine/EditorBlueprintResources/StandardMacros.IsValid` _refillhealthwb1
    (:`Is Valid`
      (`Widget.RemoveFromParent` _refillhealthwb1))))

(fn `UserConstructionScript`)