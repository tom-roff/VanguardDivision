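; Parent interactable ladder that builds itself from stacked tile meshes and teleports the player between its top and bottom.
; After BeginPlay, a timer starts a recursive spawn chain up to the set part count, then clears and offsets the top exit toward the chosen side.
; Looking at it shows a "Use Ladder" widget.
; Interaction fades to black, picks the opposite end from player height, teleports, and fades back in.
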(event `SetLadderRight`
  (bind _topofladder (`self.TopOfLadder`))
  ;[1 1 1] Custom Ladder Exit Locations
  (`SceneComponent.K2_SetRelativeLocation` _topofladder (`KismetMathLibrary.MakeVector` (+ (.x (`SceneComponent.RelativeLocation` _topofladder)) 110.0) (.y (`SceneComponent.RelativeLocation` _topofladder)) (.z (`SceneComponent.RelativeLocation` (`self.PreviousLadderPartSpawned`)))) false false))

(event `self.ReceiveBeginPlay`
  ;[1 1 1] Dynamic Ladder Part Spawning
  (bind _returnvalue (`KismetSystemLibrary.K2_SetTimerDelegate` (delegate `SpawnLadder`) 0.05 true)))

(event `SpawnLadder`
  ;[1 1 1] Dynamic Ladder Part Spawning
  (bind _returnvalue (`AddComponent|NODE_AddStaticMeshComponent-0` :`RelativeTransform` (`KismetMathLibrary.MakeTransform` (`KismetMathLibrary.MakeVector` (.x (.location (`SceneComponent.GetRelativeTransform` (`self.LadderBaseMesh`)))) (.y (.location (`SceneComponent.GetRelativeTransform` (`self.LadderBaseMesh`)))) (+ (.z (.location (`SceneComponent.GetRelativeTransform` (`self.LadderBaseMesh`)))) 85.0)) (.rotation (`SceneComponent.GetRelativeTransform` (`self.LadderBaseMesh`))) (.scale (`SceneComponent.GetRelativeTransform` (`self.LadderBaseMesh`))))))
  (bind _returnvalue_2 (`StaticMeshComponent.SetStaticMesh` _returnvalue "/Game/Geometry/Meshes/CatwalkTileset/LadderNew/Ladders_LadderTile.Ladders_LadderTile"))
  (if _returnvalue_2
    (set `self.PreviousLadderPartSpawned` _returnvalue)
    (set `self.#ofLaddersSpawned` (+ (`self.#ofLaddersSpawned`) 1))
    (if (< (`self.#ofLaddersSpawned`) (`self.#ofLadderPartsToSpawn`))
      (`self.SpawnNextLadder`))))

(event `SetLadderLeft`
  (bind _topofladder (`self.TopOfLadder`))
  ;[1 1 1] Custom Ladder Exit Locations
  (`SceneComponent.K2_SetRelativeLocation` _topofladder (`KismetMathLibrary.MakeVector` (+ (.x (`SceneComponent.RelativeLocation` _topofladder)) -130.0) (.y (`SceneComponent.RelativeLocation` _topofladder)) (.z (`SceneComponent.RelativeLocation` (`self.PreviousLadderPartSpawned`)))) false false))

(event `SpawnNextLadder`
  ;[1 1 1] Dynamic Ladder Part Spawning
  (if (< (`self.#ofLaddersSpawned`) (`self.#ofLadderPartsToSpawn`))
    (bind _returnvalue (`AddComponent|NODE_AddStaticMeshComponent-1` :`RelativeTransform` (`KismetMathLibrary.MakeTransform` (`KismetMathLibrary.MakeVector` (.x (.location (`SceneComponent.GetRelativeTransform` (`self.PreviousLadderPartSpawned`)))) (.y (.location (`SceneComponent.GetRelativeTransform` (`self.PreviousLadderPartSpawned`)))) (+ (.z (.location (`SceneComponent.GetRelativeTransform` (`self.PreviousLadderPartSpawned`)))) 85.0)) (.rotation (`SceneComponent.GetRelativeTransform` (`self.PreviousLadderPartSpawned`))) (.scale (`SceneComponent.GetRelativeTransform` (`self.PreviousLadderPartSpawned`))))))
    (bind _returnvalue_2 (`StaticMeshComponent.SetStaticMesh` _returnvalue "/Game/Geometry/Meshes/CatwalkTileset/LadderNew/Ladders_LadderTile.Ladders_LadderTile"))
    (if _returnvalue_2
      (set `self.PreviousLadderPartSpawned` _returnvalue)
      (set `self.#ofLaddersSpawned` (+ (`self.#ofLaddersSpawned`) 1))
      (if (< (`self.#ofLaddersSpawned`) (`self.#ofLadderPartsToSpawn`))
        (`self.SpawnNextLadder`)
        (else
          (`KismetSystemLibrary.K2_ClearAndInvalidateTimerHandle` (stale `self.ReceiveBeginPlay` _returnvalue))
          (switch `/Game/Blueprints/AllLevels/Variables/Enums/ExitLocations` (`self.ExitLoc`)
            (:`NewEnumerator0`
              (`self.SetLadderBack`))
            (:`NewEnumerator1`
              (`self.SetLadderFront`))
            (:`NewEnumerator2`
              (`self.SetLadderLeft`))
            (:`NewEnumerator3`
              (`self.SetLadderRight`))))))))

(event `SetLadderFront`
  (bind _topofladder (`self.TopOfLadder`))
  ;[1 1 1] Custom Ladder Exit Locations
  (`SceneComponent.K2_SetRelativeLocation` _topofladder (`KismetMathLibrary.MakeVector` (.x (`SceneComponent.RelativeLocation` _topofladder)) (+ (.y (`SceneComponent.RelativeLocation` _topofladder)) -120.0) (.z (`SceneComponent.RelativeLocation` (`self.PreviousLadderPartSpawned`)))) false false))

(event `SetLadderBack`
  (bind _topofladder (`self.TopOfLadder`))
  ;[1 1 1] Custom Ladder Exit Locations
  (`SceneComponent.K2_SetRelativeLocation` _topofladder (`KismetMathLibrary.MakeVector` (.x (`SceneComponent.RelativeLocation` _topofladder)) (+ (.y (`SceneComponent.RelativeLocation` _topofladder)) 200.0) (.z (`SceneComponent.RelativeLocation` (`self.PreviousLadderPartSpawned`)))) false false))

(event `/Game/Blueprints/Interfaces/PlayerInterface.BeginLookAt`
  (params (`Looking at Controller` :type "PlayerController Object Reference"))
  ;[1 1 1] Interact With Ladder UI
  (`/Engine/EditorBlueprintResources/StandardMacros.IsValid` (stale `/Game/Blueprints/Interfaces/PlayerInterface.BeginLookAt` _returnvalue)
    (:`Is Valid`
      _)
    (:`Is Not Valid`
      (bind _returnvalue (`|CreateWidget` "/Game/UI_elements/GameplayWBs/BaseLookingAtUI.BaseLookingAtUI_C" (`GameplayStatics.GetPlayerController` 0)))))
  (set `/Game/UI_elements/GameplayWBs/BaseLookingAtUI.TextToShow` "Use Ladder" _returnvalue)
  (`UserWidget.AddToViewport` _returnvalue -1))

(event `/Game/Blueprints/Interfaces/PlayerInterface.EndLookAt`
  (params (LookingAtController :type "PlayerController Object Reference"))
  ;[1 1 1] Interact With Ladder UI
  (`/Engine/EditorBlueprintResources/StandardMacros.IsValid` (stale `/Game/Blueprints/Interfaces/PlayerInterface.BeginLookAt` _returnvalue)
    (:`Is Valid`
      (`Widget.RemoveFromParent` (stale `/Game/Blueprints/Interfaces/PlayerInterface.BeginLookAt` _returnvalue)))))

(event `/Game/Blueprints/Interfaces/PlayerInterface.LookingAt`
  (params (LookingAtController :type "PlayerController Object Reference"))
  ;[1 1 1] Ladder Interaction
  (bind _asadvanced_sessions_game_instance_main (cast `/Game/Blueprints/AllLevels/AdvancedSessionsGameInstanceMain` (`GameplayStatics.GetGameInstance`)))
  (`/Game/Blueprints/AllLevels/AdvancedSessionsGameInstanceMain.FadeToBlack` _asadvanced_sessions_game_instance_main 1.4)
  (`KismetSystemLibrary.Delay` 1.6)
  (bind _astrue_first_person_character (cast `/Game/TrueFPP/TrueFirstPersonCharacter` (`GameplayStatics.GetPlayerCharacter` 0))
    (:`then`
      (bind _capsulecomponent (`Character.CapsuleComponent` _astrue_first_person_character))
      (if (> (.z (`SceneComponent.K2_GetComponentLocation` _capsulecomponent)) (- (.z (`SceneComponent.K2_GetComponentLocation` (`self.PreviousLadderPartSpawned`))) 100.0))
        (`SceneComponent.K2_SetWorldLocationAndRotation` _capsulecomponent (+ (.location (`SceneComponent.K2_GetComponentToWorld` (`self.BottomOfLadder`))) (0.0 0.0 100.0)) (.rotation (`SceneComponent.K2_GetComponentToWorld` (`self.BottomOfLadder`))) false true)
        (else
          (`SceneComponent.K2_SetWorldLocation` _capsulecomponent (`KismetMathLibrary.MakeVector` (.x (`SceneComponent.K2_GetComponentLocation` (`self.TopOfLadder`))) (.y (`SceneComponent.K2_GetComponentLocation` (`self.TopOfLadder`))) (+ (.z (`SceneComponent.K2_GetComponentLocation` (`self.TopOfLadder`))) 100.0)) false true)))
      (bind _asadvanced_sessions_game_instance_main_2 (cast `/Game/Blueprints/AllLevels/AdvancedSessionsGameInstanceMain` (`GameplayStatics.GetGameInstance`)))
      (`/Game/Blueprints/AllLevels/AdvancedSessionsGameInstanceMain.FadeOutOfBlack` _asadvanced_sessions_game_instance_main_2 0.6))
    (:`CastFailed`
      (`KismetSystemLibrary.PrintString` "Cast to FPP Char Failed"))))

(fn `UserConstructionScript`)