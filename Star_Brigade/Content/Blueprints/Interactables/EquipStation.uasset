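; Interactable equipment station that opens the equip station menu through the player controller.
; Look-at events show and remove an "Equipment Station" interact prompt, while Lookingat creates the menu UI.
; A looping timer begins Sparks trails at an interval randomized once at BeginPlay.
; A second looping timer re-rolls a Random variable, which does not feed the spark timer.
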(event `self.ReceiveBeginPlay`
  (`KismetSystemLibrary.K2_SetTimerDelegate` (delegate `SetRandom#`) 2.0 true)
  (`KismetSystemLibrary.K2_SetTimerDelegate` (delegate `SpawnSparks`) (`KismetMathLibrary.RandomFloatInRange` 2.0 5.0) true))

(event `SetRandom#`
  (set `self.Random#` (`KismetMathLibrary.RandomFloatInRange` 2.0 5.0)))

(event `SpawnSparks`
  (`ParticleSystemComponent.BeginTrails` (`self.Sparks`) "None" "None" "ETrailWidthMode_FromCentre" 0.0))

(event `/Game/Blueprints/Interfaces/PlayerInterface.LookingAt`
  (params (LookingAtController :type "PlayerController Object Reference"))
  (bind _asplayer_controller_main (cast `/Game/Blueprints/AllLevels/PlayerControllerMain` LookingAtController))
  (`/Game/Blueprints/AllLevels/PlayerControllerMain.CreateMenuUI` _asplayer_controller_main "/Game/UI_elements/Stations/EquipStationUI.EquipStationUI_C"))

(event `/Game/Blueprints/Interfaces/PlayerInterface.BeginLookAt`
  (params (`Looking at Controller` :type "PlayerController Object Reference"))
  (`/Engine/EditorBlueprintResources/StandardMacros.IsValid` `Looking at Controller`
    (:`Is Valid`
      (`/Game/Blueprints/WidgetFuncs.ShowInteractWB` "Equipment Station" (cast `/Game/Blueprints/AllLevels/PlayerControllerMain` `Looking at Controller` :!pure true)))))

(event `/Game/Blueprints/Interfaces/PlayerInterface.EndLookAt`
  (params (LookingAtController :type "PlayerController Object Reference"))
  (`/Engine/EditorBlueprintResources/StandardMacros.IsValid` LookingAtController
    (:`Is Valid`
      (`/Game/Blueprints/AllLevels/PlayerControllerMain.RemoveInteractWB` (cast `/Game/Blueprints/AllLevels/PlayerControllerMain` LookingAtController :!pure true)))))

(fn `UserConstructionScript`)