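; Base interactable upgrade station that gives players access to an upgrade menu through look-at events.
; BeginLookat has PlayerControllerMain show an "Upgrade Station" interact prompt and stores the widget, which EndLookat removes.
; Lookingat has the controller create the UpgradeStationBase menu and records it in a unique list of looking controllers.
; The CanUseStation check has empty branches, so it does not restrict use.
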(event `/Game/Blueprints/Interfaces/PlayerInterface.EndLookAt`
  (params (LookingAtController :type "PlayerController Object Reference"))
  (bind _addedwb (`self.AddedWB`))
  (`/Engine/EditorBlueprintResources/StandardMacros.IsValid` _addedwb
    (:`Is Valid`
      (`Widget.RemoveFromParent` _addedwb))))

(event `/Game/Blueprints/Interfaces/PlayerInterface.BeginLookAt`
  (params (`Looking at Controller` :type "PlayerController Object Reference"))
  (bind _asplayer_controller_main (cast `/Game/Blueprints/AllLevels/PlayerControllerMain` `Looking at Controller` :!pure true))
  (`/Engine/EditorBlueprintResources/StandardMacros.IsValid` _asplayer_controller_main
    (:`Is Valid`
      (bind _wb_created (`/Game/Blueprints/AllLevels/PlayerControllerMain.ShowInteractWB` _asplayer_controller_main "Upgrade Station"))
      (set `self.AddedWB` _wb_created))))

(event `/Game/Blueprints/Interfaces/PlayerInterface.LookingAt`
  (params (LookingAtController :type "PlayerController Object Reference"))
  (if (`self.CanUseStation?`)
    _
    (else
      _))
  (bind _asplayer_controller_main (cast `/Game/Blueprints/AllLevels/PlayerControllerMain` LookingAtController))
  (`/Game/Blueprints/AllLevels/PlayerControllerMain.CreateMenuUI` _asplayer_controller_main "/Game/UI_elements/WaveModeUI/BaseUpgradeStation/UpgradeStationBase.UpgradeStationBase_C")
  (`KismetArrayLibrary.Array_AddUnique` (`self.LookingAtControllers`) _asplayer_controller_main))

(fn `UserConstructionScript`)