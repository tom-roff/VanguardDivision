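; Base interactable ladder Blueprint that instantly moves the player character between the top and bottom of the ladder.
; The Lookingat event branches on authority, calling MoveUpLadder directly or through MoveUpLadderClient when remote.
; MoveUpLadder compares player 0's height to a hard-coded world Z, then sets its location to the BottomOfLadder or TopOfLadder component without sweeping.
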(event `MoveUpLadderClient`
  (`self.Move Up Ladder`))

(event `/Game/Blueprints/Interfaces/PlayerInterface.LookingAt`
  (params (LookingAtController :type "PlayerController Object Reference"))
  (`/Engine/EditorBlueprintResources/ActorMacros.Switch Has Authority`
    (:`Authority`
      (`self.Move Up Ladder`))
    (:`Remote`
      (`self.MoveUpLadderClient`))))

(event `Move Up Ladder`
  (bind _returnvalue (`GameplayStatics.GetPlayerCharacter` 0))
  (if (> (.z (`self.K2_GetActorLocation` (`GameplayStatics.GetPlayerCharacter` 0))) 948.0)
    (`self.K2_SetActorLocation` _returnvalue (`SceneComponent.K2_GetComponentLocation` (`self.Bottom of Ladder`)) false false)
    (else
      (`self.K2_SetActorLocation` _returnvalue (`SceneComponent.K2_GetComponentLocation` (`self.Top of Ladder`)) false false))))

(fn `UserConstructionScript`)