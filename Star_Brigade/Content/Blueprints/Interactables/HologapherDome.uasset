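; Deployable shield dome ability owned by a TrueFirstPersonCharacter, with its own health pool and perk-driven bonuses.
; On BeginPlay it sets shield health, doubled by one perk; damage drains it until the owner's RemoveDome is called.
; With another perk, any mesh overlap starts a looping timer that heals the owner, cleared on end overlap.
; On destruction it removes the dome UI and decrements the owner's deployed-ability count.
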(event `self.ReceiveDestroyed`
  (bind _asplayer_controller_main (cast `/Game/Blueprints/AllLevels/PlayerControllerMain` (`Pawn.GetController` (cast `Pawn` (`self.GetOwner`) :!pure true)))
    (:`then`
      (`/Game/Blueprints/AllLevels/PlayerControllerMain.RemoveDomeUI` _asplayer_controller_main))
    (:`CastFailed`
      _))
  (bind _astrue_first_person_character (cast `/Game/TrueFPP/TrueFirstPersonCharacter` (`self.GetOwner`)))
  (set `/Game/TrueFPP/TrueFirstPersonCharacter.AbilitiesDeployed` (- (`/Game/TrueFPP/TrueFirstPersonCharacter.AbilitiesDeployed` _astrue_first_person_character) 1) _astrue_first_person_character))

(event `self.Mesh.OnComponentBeginOverlap`
  (params (OverlappedComponent :type "PrimitiveComponent Object Reference") (OtherActor :type "Actor Object Reference") (OtherComp :type "PrimitiveComponent Object Reference") (OtherBodyIndex :type Integer) (bFromSweep :type Boolean) (SweepResult :type "HitResult Structure (by ref)"))
  ;[1 1 1] Medical Dome Handling
  (bind _astrue_first_person_character (cast `/Game/TrueFPP/TrueFirstPersonCharacter` (`self.GetOwner`)))
  (if (not (== (`KismetArrayLibrary.Array_Find` (`/Game/TrueFPP/TrueFirstPersonCharacter.PurchasedPerks` _astrue_first_person_character) "NewEnumerator12") -1))
    (bind _returnvalue (`KismetSystemLibrary.K2_SetTimerDelegate` (delegate `SetHealTimer`) 1.1 true))
    (set `self.HealTimer` _returnvalue)))

(event `SetHealTimer`
  ;[1 1 1] Medical Dome Handling
  (`/Game/TrueFPP/TrueFirstPersonCharacter.HealPlayer` (stale `self.Mesh.OnComponentBeginOverlap` _astrue_first_person_character) 2))

(event `SetDomeHealthServer`
  ;[1 1 1] When the dome begins existing, set the shield health depending on player perks
  (bind _astrue_first_person_character (cast `/Game/TrueFPP/TrueFirstPersonCharacter` (`self.GetOwner`)))
  (if (== (`KismetArrayLibrary.Array_Find` (`/Game/TrueFPP/TrueFirstPersonCharacter.PurchasedPerks` _astrue_first_person_character) "NewEnumerator13") -1)
    (set `self.ShieldHealth` (`self.NormalMaxShieldHealth`))
    (else
      (bind _output_get (set `self.ShieldHealth` (* (`self.NormalMaxShieldHealth`) 2.0)))
      (set `self.MaxShieldHealth` _output_get))))

(event `self.ReceiveBeginPlay`
  ;[1 1 1] When the dome begins existing, set the shield health depending on player perks
  (`self.SetDomeHealthServer`))

(event `self.Mesh.OnComponentEndOverlap`
  (params (OverlappedComponent :type "PrimitiveComponent Object Reference") (OtherActor :type "Actor Object Reference") (OtherComp :type "PrimitiveComponent Object Reference") (OtherBodyIndex :type Integer))
  ;[1 1 1] Medical Dome Handling
  (`KismetSystemLibrary.K2_ClearAndInvalidateTimerHandle` (`self.HealTimer`)))

(event `self.ReceiveAnyDamage`
  (params (Damage :type "Float (single-precision)") (DamageType :type "DamageType Object Reference") (InstigatedBy :type "Controller Object Reference") (DamageCauser :type "Actor Object Reference"))
  ;[1 1 1] Dome Health Management
  (bind _output_get (set `self.ShieldHealth` (- (`self.ShieldHealth`) Damage)))
  (if (<= _output_get 0.0)
    (bind _astrue_first_person_character (cast `/Game/TrueFPP/TrueFirstPersonCharacter` (`self.GetOwner`)))
    (`/Game/TrueFPP/TrueFirstPersonCharacter.RemoveDome` _astrue_first_person_character)))

(fn `UserConstructionScript`
  (`parent.UserConstructionScript`))