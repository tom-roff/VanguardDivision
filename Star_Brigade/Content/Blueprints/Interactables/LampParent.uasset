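; Parent Blueprint for interactable lamps that the player toggles on and off through look-at interaction events.
; BeginLookat and EndLookat show and remove a "Toggle Light" prompt on PlayerControllerMain.
; Lookingat calls ServerToggle, which flips IsOn, switches PointLight1 intensity between zero and IntensityBrightness, and plays an attenuated switch sound.
; The construction script applies IntensityBrightness to the light.
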(event `/Game/Blueprints/Interfaces/PlayerInterface.LookingAt`
  (params (LookingAtController :type "PlayerController Object Reference"))
  ;[1 1 1] On/Off Functionality
  (`self.ServerToggle`))

(event `/Game/Blueprints/Interfaces/PlayerInterface.BeginLookAt`
  (params (`Looking at Controller` :type "PlayerController Object Reference"))
  ;[1 1 1] Create Toggle Light Widget when player looks at Object
  (bind _asplayer_controller_main (cast `/Game/Blueprints/AllLevels/PlayerControllerMain` `Looking at Controller`))
  (`/Game/Blueprints/AllLevels/PlayerControllerMain.ShowInteractWB` _asplayer_controller_main "Toggle Light"))

(event `ServerToggle`
  ;[1 1 1] On/Off Functionality
  (if (`self.IsOn?`)
    (`LightComponent.SetIntensity` (`self.PointLight1`) 0.0)
    (set `self.IsOn?` false)
    (else
      (`LightComponent.SetIntensity` (`self.PointLight1`) (`self.Intensity/Brightness`))
      (set `self.IsOn?` true)))
  (`GameplayStatics.PlaySoundAtLocation` "/Game/Audio/switchgood.switchgood" (`self.K2_GetActorLocation`) (struct) 1.0 1.0 0.0 "/Game/Audio/Attenuations/SmallSoundsAtten.SmallSoundsAtten" null null))

(event `/Game/Blueprints/Interfaces/PlayerInterface.EndLookAt`
  (params (LookingAtController :type "PlayerController Object Reference"))
  ;[1 1 1] Remove when player stops looking at object
  (bind _asplayer_controller_main (cast `/Game/Blueprints/AllLevels/PlayerControllerMain` LookingAtController))
  (`/Game/Blueprints/AllLevels/PlayerControllerMain.RemoveInteractWB` _asplayer_controller_main))

(event `self.ReceiveBeginPlay`
  ;[1 1 1] On Play, Set Intensity to desired value (set in variable)
)

(fn `UserConstructionScript`
  (`LightComponent.SetIntensity` (`self.PointLight1`) (`self.Intensity/Brightness`)))