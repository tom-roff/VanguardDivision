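; AmmoBox is an interactable ammo pickup that refills all ammo for the TrueFirstPersonCharacter interacting with it.
; A looping timer steadily spins its AmmoRot component around yaw, rather than using Tick.
; BeginLookat and EndLookat show and hide a cached "Refill Ammo" prompt widget.
; Lookingat calls the current weapon's ammo update message, refills all ammo and plays a beep, without consuming the box.
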(event `self.ReceiveBeginPlay`
  ;[1 1 1] Mesh Rotation
  (`KismetSystemLibrary.K2_SetTimerDelegate` (delegate `RotMesh`) 0.025 true))

(event `RotMesh`
  ;[1 1 1] Mesh Rotation
  (`SceneComponent.K2_SetWorldRotation` (`self.AmmoRot`) (`KismetMathLibrary.MakeRotator` 0.0 0.0 (+ (.yaw (`SceneComponent.K2_GetComponentRotation` (`self.AmmoRot`))) 1.0)) false false))

(event `/Game/Blueprints/Interfaces/PlayerInterface.LookingAt`
  (params (LookingAtController :type "PlayerController Object Reference"))
  (bind _astrue_first_person_character (cast `/Game/TrueFPP/TrueFirstPersonCharacter` (`Controller.K2_GetPawn` LookingAtController)))
  (message `/Game/Blueprints/Interfaces/AmmoInterface.AmmoUpdate` (`/Game/TrueFPP/TrueFirstPersonCharacter.CurrentWeaponInHand` _astrue_first_person_character))
  (`/Game/TrueFPP/TrueFirstPersonCharacter.RefillAllAmmos` _astrue_first_person_character)
  (`GameplayStatics.PlaySound2D` "/Game/Audio/UISounds/Beep2Low.Beep2Low" 1.0 1.0 0.0 null null))

(event `/Game/Blueprints/Interfaces/PlayerInterface.BeginLookAt`
  (params (`Looking at Controller` :type "PlayerController Object Reference"))
  (`/Engine/EditorBlueprintResources/StandardMacros.IsValid` (`self.RefillAmmoWB1`)
    (:`Is Valid`
      _)
    (:`Is Not Valid`
      (bind _returnvalue (`|CreateWidget` "/Game/UI_elements/GameplayWBs/BaseLookingAtUI.BaseLookingAtUI_C" (`GameplayStatics.GetPlayerController` 0)))
      (set `self.RefillAmmoWB1` _returnvalue)))
  (set `/Game/UI_elements/GameplayWBs/BaseLookingAtUI.TextToShow` "Refill Ammo" (`self.RefillAmmoWB1`))
  (`UserWidget.AddToViewport` (`self.RefillAmmoWB1`) 0))

(event `/Game/Blueprints/Interfaces/PlayerInterface.EndLookAt`
  (params (LookingAtController :type "PlayerController Object Reference"))
  (bind _refillammowb1 (`self.RefillAmmoWB1`))
  (`/Engine/EditorBlueprintResources/StandardMacros.IsValid` _refillammowb1
    (:`Is Valid`
      (`Widget.RemoveFromParent` _refillammowb1))))

(fn `UserConstructionScript`)