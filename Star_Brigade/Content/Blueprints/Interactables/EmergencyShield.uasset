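; EmergencyShield is an interactable actor that knocks back nearby enemies as soon as it spawns.
; On BeginPlay it gathers EnemyParent actors overlapping its Sphere component.
; Each enemy's movement is stopped, then it is launched away from the shield with an upward boost, overriding its existing velocity.
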(event `self.ReceiveBeginPlay`
  (for _array_element (`PrimitiveComponent.GetOverlappingActors` (`self.Sphere`) "/Game/Blueprints/AIActorsPawns/EnemyParent.EnemyParent_C")
    (bind _ascharacter (cast `Character` _array_element :!pure true))
    (`MovementComponent.StopMovementImmediately` (`Character.CharacterMovement` _ascharacter))
    (`Character.LaunchCharacter` _ascharacter (+ (* (`KismetMathLibrary.GetForwardVector` (`KismetMathLibrary.FindLookAtRotation` (`self.K2_GetActorLocation`) (`self.K2_GetActorLocation` _array_element))) 2000.0) (0.0 0.0 500.0)) true true)))

(fn `UserConstructionScript`
  (`parent.UserConstructionScript`))